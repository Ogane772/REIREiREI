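; Castle actor that spawns Yusya (hero) characters on a timed schedule during the main game.
; BeginPlay copies the spawn DataTable into parallel arrays, only for the KODAI era.
; Once standby ends, Tick restarts the clock and spawns the next entry in a box when elapsed whole seconds exactly equal its time, passing stats and AI order.
; Only type 0 spawns and advances the index; Tick stops after the last entry.
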(event EventBeginPlay
  (Variables|Default|SetStartTime (Math|DateTime|Now))
  (bind _asglobal_instance (Utilities|Casting|CastToGlobalInstance (Game|GetGameInstance)))
  (switch Utilities|FlowControl|Switch|SwitchonJidaiEnum (Variables|/Game/Main/GlobalInstance.GlobalInstance_C|GetMainGameJidaiEnum _asglobal_instance)
    (:NewEnumerator0
      (bind _outrownames (DataTable|GetDataTableRowNames "/Game/Main/CSV/KodaiYusyaSpawnData.KodaiYusyaSpawnData"))
      (for (_array_element _array_index) _outrownames
        (bind _returnvalue (Utilities|GetDataTableRow "/Game/Main/CSV/KodaiYusyaSpawnData.KodaiYusyaSpawnData" _array_element)
          (:then
            (Utilities|Array|SetArrayElem (Variables|Default|GetSpawmTime) _array_index (.SpwnTime (Utilities|Struct|BreakYusyaSpawnTable _returnvalue)) true)
            (Utilities|Array|SetArrayElem (Variables|Default|GetYusyaType) _array_index (.YusyaType (Utilities|Struct|BreakYusyaSpawnTable _returnvalue)) true)
            (Utilities|Array|SetArrayElem (Variables|Default|GetYusyaAIType) _array_index (.YusyaAI_Type (Utilities|Struct|BreakYusyaSpawnTable _returnvalue)) true)
            (Utilities|Array|SetArrayElem (Variables|Default|GetHP) _array_index (.HP (Utilities|Struct|BreakYusyaSpawnTable _returnvalue)) true)
            (Utilities|Array|SetArrayElem (Variables|Default|GetATK) _array_index (.ATK (Utilities|Struct|BreakYusyaSpawnTable _returnvalue)) true)
            (Utilities|Array|SetArrayElem (Variables|Default|GetMoveSpeed) _array_index (.MoveSpeed (Utilities|Struct|BreakYusyaSpawnTable _returnvalue)) true)))))))

(event Collision|EventActorBeginOverlap
  (params (OtherActor :type Actor%20Object%20Reference)))

(event EventTick
  (params (DeltaSeconds :type Float%20%28single-precision%29))
  (bind _yusyaspawnbox (Variables|Default|GetYusyaSpawnBox))
  (bind (_origin _boxextent) (Collision|GetComponentBounds _yusyaspawnbox))
  (bind _asglobal_instance (Utilities|Casting|CastToGlobalInstance (Game|GetGameInstance)))
  (if (not (Variables|/Game/Main/GlobalInstance.GlobalInstance_C|GetIsStandby _asglobal_instance))
    (Utilities|FlowControl|Sequence
      (:then_0
        (Utilities|FlowControl|DoOnce false
          (:Completed
            (Variables|Default|SetStartTime (Math|DateTime|Now)))))
      (:then_1
        (if (Utilities|Array|IsValidIndex (Variables|Default|GetSpawmTime) (Variables|Default|GetIndexCounter))
          (bind _output_get (Variables|Default|SetSecond (Math|Timespan|GetSeconds (- (Math|DateTime|Now) (Variables|Default|GetStartTime)))))
          (bind _output_get_2 (Variables|Default|SetMinutes (* (Math|Timespan|GetMinutes (- (Math|DateTime|Now) (Variables|Default|GetStartTime))) 60)))
          (bind _output_get_3 (Variables|Default|SetNumSecond (+ _output_get_2 _output_get)))
          (if (== _output_get_3 (Utilities|Array|Get(acopy) (Variables|Default|GetSpawmTime) (Variables|Default|GetIndexCounter))) ; SpawnTableと時間が一致したら生成
            (switch int (Utilities|Array|Get(acopy) (Variables|Default|GetYusyaAIType) (Variables|Default|GetIndexCounter))
              (:0
                (Variables|Default|SetAI_TYPE "NewEnumerator0"))
              (:1
                (Variables|Default|SetAI_TYPE "NewEnumerator1"))
              (:2
                (Variables|Default|SetAI_TYPE "NewEnumerator2")))
            (switch int (Utilities|Array|Get(acopy) (Variables|Default|GetYusyaType) (Variables|Default|GetIndexCounter))
              (:0
                (Variables|Default|SetYUSYA_TYPE "NewEnumerator0")
                (Game|SpawnActorfromClass "/Game/Main/Blueprints/Yusya/Yusya01.Yusya01_C" (Math|Transform|MakeTransform (Math|Random|RandomPointinBoundingBox _origin _boxextent) "0,180.000000, 0" "1,1,1") "Undefined" 0 (Utilities|Array|Get(acopy) (Variables|Default|GetHP) (Variables|Default|GetIndexCounter)) (Utilities|Array|Get(acopy) (Variables|Default|GetATK) (Variables|Default|GetIndexCounter)) (Utilities|Array|Get(acopy) (Variables|Default|GetMoveSpeed) (Variables|Default|GetIndexCounter)) (Variables|Default|GetAI_TYPE) 0)
                (bind _result (Math|Integer|IncrementInt (Variables|Default|GetIndexCounter))
                  (:%20%20
                    (Variables|Default|SetIndexCounter _result))))))
          (else
            (Actor|Tick|SetActorTickEnabled false)))))))

(fn ConstructionScript)

(fn SetTick
  (params (Type :type Boolean))
  (Actor|Tick|SetActorTickEnabled Type))