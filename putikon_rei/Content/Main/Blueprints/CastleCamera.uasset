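; Castle camera actor that lets the player toggle the view between the main gameplay camera and itself.
; Pressing L or the gamepad left face button acts only while the GlobalInstance CastleCameraON flag is set.
; A SetCamera boolean alternates between making this actor the view target and calling CameraON on MainGameInputActor instances to hand the view back.
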(event EventBeginPlay)

(event Collision|EventActorBeginOverlap
  (params (OtherActor :type Actor%20Object%20Reference)))

(event EventTick
  (params (DeltaSeconds :type Float%20%28single-precision%29)))

(event Input|GamepadEvents|GamepadFaceButtonLeft
  (params (Key :type Key%20Structure))
  (:Pressed
    (if (Variables|/Game/Main/GlobalInstance.GlobalInstance_C|GetCastleCameraON (.AsGlobal%20Instance (Utilities|Casting|CastToGlobalInstance (Game|GetGameInstance))))
      (if (Variables|Default|GetSetCamera)
        (bind _outactors (Actor|GetAllActorsOfClass "/Game/Main/Blueprints/MainGameInputActor.MainGameInputActor_C"))
        (Default|CameraON _outactors)
        (Variables|Default|SetSetCamera false)
        (else
          (Game|Player|SetViewTargetwithBlend (Game|GetPlayerController 0) self 0.0 "VTBlend_Linear" 0.0 false)
          (Variables|Default|SetSetCamera true))))))

(event Input|KeyboardEvents|L
  (params (Key :type Key%20Structure))
  (:Pressed
    (if (Variables|/Game/Main/GlobalInstance.GlobalInstance_C|GetCastleCameraON (.AsGlobal%20Instance (Utilities|Casting|CastToGlobalInstance (Game|GetGameInstance))))
      (if (Variables|Default|GetSetCamera)
        (bind _outactors (Actor|GetAllActorsOfClass "/Game/Main/Blueprints/MainGameInputActor.MainGameInputActor_C"))
        (Default|CameraON _outactors)
        (Variables|Default|SetSetCamera false)
        (else
          (Game|Player|SetViewTargetwithBlend (Game|GetPlayerController 0) self 0.0 "VTBlend_Linear" 0.0 false)
          (Variables|Default|SetSetCamera true))))))

(fn ConstructionScript)