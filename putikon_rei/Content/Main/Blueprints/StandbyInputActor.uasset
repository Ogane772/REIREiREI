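; Input actor for the pre-game standby screen, where the player places, replaces or removes enemy nests before starting.
; BeginPlay creates StandbyUI and fills it by matching KodaiNestData rows to EnemyData.
; Gamepad and keyboard share cursor logic, switched by TitleMode, NestTips and NestON flags, driving StandbyUI, NestPointBP markers and UMGActor2DCapture previews.
; EndPlay removes the UI, passes a nest count to MainGameInputActor and clears GlobalInstance's standby flag.
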(event EventBeginPlay
  (bind _asglobal_instance (Utilities|Casting|CastToGlobalInstance (Game|GetGameInstance)))
  (Variables|/Game/Main/GlobalInstance.GlobalInstance_C|SetMainGameJidaiEnum _asglobal_instance "NewEnumerator0")
  (bind _returnvalue (UserInterface|CreateWidget "/Game/Main/UI/StandbyUI.StandbyUI_C"))
  (bind _output_get (Variables|Default|SetStandbyUI _returnvalue))
  (UserInterface|Viewport|AddtoViewport _output_get 0)
  (switch Utilities|FlowControl|Switch|SwitchonJidaiEnum (Variables|/Game/Main/GlobalInstance.GlobalInstance_C|GetMainGameJidaiEnum _asglobal_instance)
    (:NewEnumerator0
      (bind _outrownames (DataTable|GetDataTableRowNames "/Game/Main/CSV/KodaiNestData.KodaiNestData"))
      (for _array_element _outrownames
        (bind _returnvalue_2 (Utilities|GetDataTableRow "/Game/Main/CSV/KodaiNestData.KodaiNestData" _array_element)
          (:then
            (bind _outrownames_2 (DataTable|GetDataTableRowNames "/Game/Main/CSV/EnemyData.EnemyData"))
            (for _array_element_2 _outrownames_2
              (bind _returnvalue_3 (Utilities|GetDataTableRow "/Game/Main/CSV/EnemyData.EnemyData" _array_element_2)
                (:then
                  (if (== (.Number (Utilities|Struct|BreakEnemyDataTable _returnvalue_3)) (Utilities|Struct|BreakKodaiNestDataTable _returnvalue_2))
                    (Default|SetNestData (Variables|Default|GetStandbyUI) (Utilities|String|ToString(Text) (.Name (Utilities|Struct|BreakEnemyDataTable _returnvalue_3))) (.HP (Utilities|Struct|BreakEnemyDataTable _returnvalue_3)) (.ATK (Utilities|Struct|BreakEnemyDataTable _returnvalue_3)) (.MoveSpeed (Utilities|Struct|BreakEnemyDataTable _returnvalue_3)) (.AttackType (Utilities|Struct|BreakEnemyDataTable _returnvalue_3)) (.MAXNUM (Utilities|Struct|BreakEnemyDataTable _returnvalue_3)) (.Number (Utilities|Struct|BreakEnemyDataTable _returnvalue_3))))))))))
      (bind _nestnum (Default|GetNestNum (Variables|Default|GetStandbyUI)))
      (Variables|Default|SetNestNum _nestnum)
      (Default|SetCursorNumber (Variables|Default|GetStandbyUI)))))

(event Collision|EventActorBeginOverlap
  (params (OtherActor :type Actor%20Object%20Reference))
  ;[1 1 1] 左ウィンドウ操作
)

(event EventEndPlay
  (params (EndPlayReason :type EEndPlayReason%20Enum :default "Destroyed"))
  (Variables|Default|SetNestCount (Variables|/Game/Main/UI/StandbyUI.StandbyUI_C|GetNestCounter (Variables|Default|GetStandbyUI)))
  (Widget|RemovefromParent (Variables|Default|GetStandbyUI))
  (bind _outactors (Actor|GetAllActorsOfClass "/Game/Main/Blueprints/MainGameInputActor.MainGameInputActor_C"))
  (for _array_element _outactors
    (bind _result (Math|Integer|DecrementInt (Variables|Default|GetNestCount))
      (:%20%20
        (Default|SetNestNum _array_element _result))))
  (bind _asglobal_instance (Utilities|Casting|CastToGlobalInstance (Game|GetGameInstance)))
  (Variables|/Game/Main/GlobalInstance.GlobalInstance_C|SetIsStandby _asglobal_instance false))

(event EventTick
  (params (DeltaSeconds :type Float%20%28single-precision%29)))

(event Input|GamepadEvents|GamepadLeftStickUp
  (params (Key :type Key%20Structure))
  ;[1 1 1] 左ウィンドウ操作
  (:Pressed
    (if (Class|KismetInputLibrary|KeyIsValid Key)
      (if (not (Variables|/Game/Main/UI/StandbyUI.StandbyUI_C|GetNoInput (Variables|Default|GetStandbyUI)))
        (if (not (Variables|Default|GetTitleMode))
          (if (not (Variables|Default|GetNestTips))
            (bind _result (Math|Integer|DecrementInt (Variables|Default|GetCursorNumber))
              (:%20%20
                (if (< _result 0)
                  (bind _output_get (Variables|Default|SetCursorNumber 2))
                  (Default|SetCursorNumber (Variables|Default|GetStandbyUI) _output_get)
                  (else
                    (bind _output_get_2 (Variables|Default|SetCursorNumber _result))
                    (Default|SetCursorNumber (Variables|Default|GetStandbyUI) _output_get_2)))))))))))

(event Input|GamepadEvents|GamepadLeftStickDown
  (params (Key :type Key%20Structure))
  ;[1 1 1] 左ウィンドウ操作
  (:Pressed
    (if (Class|KismetInputLibrary|KeyIsValid Key)
      (if (not (Variables|/Game/Main/UI/StandbyUI.StandbyUI_C|GetNoInput (Variables|Default|GetStandbyUI)))
        (if (not (Variables|Default|GetTitleMode))
          (if (not (Variables|Default|GetNestTips))
            (bind _result (Math|Integer|IncrementInt (Variables|Default|GetCursorNumber))
              (:%20%20
                (if (> _result 2)
                  (bind _output_get (Variables|Default|SetCursorNumber 0))
                  (Default|SetCursorNumber (Variables|Default|GetStandbyUI) _output_get)
                  (else
                    (bind _output_get_2 (Variables|Default|SetCursorNumber _result))
                    (Default|SetCursorNumber (Variables|Default|GetStandbyUI) _output_get_2)))))))))))

(event Input|GamepadEvents|GamepadLeftStickLeft
  (params (Key :type Key%20Structure))
  (bind _standbyui (Variables|Default|GetStandbyUI))
  (bind _standbyui_2 (Variables|Default|GetStandbyUI))
  ;[1 1 1] 右ウィンドウAnd巣を設置操作
  (:Pressed
    (if (Class|KismetInputLibrary|KeyIsValid Key)
      (if (not (Variables|/Game/Main/UI/StandbyUI.StandbyUI_C|GetNoInput (Variables|Default|GetStandbyUI)))
        (if (Variables|Default|GetTitleMode)
          (Variables|Default|SetCursorNumber 0)
          (Default|SetCursorNumber (Variables|Default|GetStandbyUI))
          (elif (Variables|Default|GetNestTips)
            (if (Variables|Default|GetNestON)
              (Variables|Default|SetTimeCursorNumber (Variables|Default|GetCursorNumber))
              (bind _result (Math|Integer|DecrementInt (Variables|Default|GetCursorNumber))
                (:%20%20
                  (if (< _result 0)
                    (bind _output_get (Variables|Default|SetCursorNumber (- (Variables|Default|GetNestPointNum) 1)))
                    (Default|SetCursorNumber (Variables|Default|GetStandbyUI) _output_get)
                    (else
                      (bind _output_get_2 (Variables|Default|SetCursorNumber _result))
                      (Default|SetCursorNumber (Variables|Default|GetStandbyUI) _output_get_2)))
                  (bind _outactors (Actor|GetAllActorsOfClass "/Game/Main/Blueprints/NestPointBP.NestPointBP_C"))
                  (for _array_element _outactors
                    (if (== (Variables|Default|GetCursorNumber) (Variables|/Game/Main/Blueprints/NestPointBP.NestPointBP_C|GetPointNumber _array_element))
                      (Default|SetYajirusiVisi _array_element true)
                      (bind _neston (Default|GetNestON _array_element))
                      (Default|SetNestCheck (Variables|Default|GetStandbyUI) _neston)
                      (elif (== (Variables|/Game/Main/Blueprints/NestPointBP.NestPointBP_C|GetPointNumber _array_element) (Variables|Default|GetTimeCursorNumber))
                        (Default|SetYajirusiVisi _array_element false))))))
              (else
                (bind _result_2 (Math|Integer|DecrementInt (Variables|Default|GetCursorNumber))
                  (:%20%20
                    (if (< _result_2 0)
                      (bind _output_get_3 (Variables|Default|SetCursorNumber 2))
                      (Default|SetCursorNumber _standbyui _output_get_3)
                      (bind _enemytype (Default|GetEnemyType _standbyui _output_get_3))
                      (bind _outactors_2 (Actor|GetAllActorsOfClass "/Game/Main/UI/UMGActor2DCapture.UMGActor2DCapture_C"))
                      (for _array_element_2 _outactors_2
                        (Default|SetEnemyType _array_element_2 _enemytype)
                        (Default|SetCursorAnime (Variables|Default|GetStandbyUI) false))
                      (else
                        (bind _output_get_4 (Variables|Default|SetCursorNumber _result_2))
                        (Default|SetCursorNumber _standbyui_2 _output_get_4)
                        (bind _enemytype_2 (Default|GetEnemyType _standbyui_2 _output_get_4))
                        (bind _outactors_3 (Actor|GetAllActorsOfClass "/Game/Main/UI/UMGActor2DCapture.UMGActor2DCapture_C"))
                        (for _array_element_3 _outactors_3
                          (Default|SetEnemyType _array_element_3 _enemytype_2)
                          (Default|SetCursorAnime (Variables|Default|GetStandbyUI) false))))))))))))))

(event Input|KeyboardEvents|D
  (params (Key :type Key%20Structure))
  (bind _standbyui (Variables|Default|GetStandbyUI))
  (bind _standbyui_2 (Variables|Default|GetStandbyUI))
  ;[1 1 1] 右ウィンドウAnd巣を設置操作
  (:Pressed
    (if (not (Variables|/Game/Main/UI/StandbyUI.StandbyUI_C|GetNoInput (Variables|Default|GetStandbyUI)))
      (if (Variables|Default|GetTitleMode)
        (bind _output_get (Variables|Default|SetCursorNumber 1))
        (Default|SetCursorNumber (Variables|Default|GetStandbyUI) _output_get)
        (elif (Variables|Default|GetNestTips)
          (if (Variables|Default|GetNestON)
            (Variables|Default|SetTimeCursorNumber (Variables|Default|GetCursorNumber))
            (bind _result (Math|Integer|IncrementInt (Variables|Default|GetCursorNumber))
              (:%20%20
                (if (> _result (- (Variables|Default|GetNestPointNum) 1))
                  (bind _output_get_2 (Variables|Default|SetCursorNumber 0))
                  (Default|SetCursorNumber (Variables|Default|GetStandbyUI) _output_get_2)
                  (else
                    (bind _output_get_3 (Variables|Default|SetCursorNumber _result))
                    (Default|SetCursorNumber (Variables|Default|GetStandbyUI) _output_get_3)))
                (bind _outactors (Actor|GetAllActorsOfClass "/Game/Main/Blueprints/NestPointBP.NestPointBP_C"))
                (for _array_element _outactors
                  (if (== (Variables|Default|GetCursorNumber) (Variables|/Game/Main/Blueprints/NestPointBP.NestPointBP_C|GetPointNumber _array_element))
                    (Default|SetYajirusiVisi _array_element true)
                    (bind _neston (Default|GetNestON _array_element))
                    (Default|SetNestCheck (Variables|Default|GetStandbyUI) _neston)
                    (elif (== (Variables|/Game/Main/Blueprints/NestPointBP.NestPointBP_C|GetPointNumber _array_element) (Variables|Default|GetTimeCursorNumber))
                      (Default|SetYajirusiVisi _array_element false))))))
            (else
              (bind _result_2 (Math|Integer|IncrementInt (Variables|Default|GetCursorNumber))
                (:%20%20
                  (if (> _result_2 2)
                    (bind _output_get_4 (Variables|Default|SetCursorNumber 0))
                    (Default|SetCursorNumber _standbyui _output_get_4)
                    (bind _enemytype (Default|GetEnemyType _standbyui _output_get_4))
                    (bind _outactors_2 (Actor|GetAllActorsOfClass "/Game/Main/UI/UMGActor2DCapture.UMGActor2DCapture_C"))
                    (for _array_element_2 _outactors_2
                      (Default|SetEnemyType _array_element_2 _enemytype)
                      (Default|SetCursorAnime (Variables|Default|GetStandbyUI) true))
                    (else
                      (bind _output_get_5 (Variables|Default|SetCursorNumber _result_2))
                      (Default|SetCursorNumber _standbyui_2 _output_get_5)
                      (bind _enemytype_2 (Default|GetEnemyType _standbyui_2 _output_get_5))
                      (bind _outactors_3 (Actor|GetAllActorsOfClass "/Game/Main/UI/UMGActor2DCapture.UMGActor2DCapture_C"))
                      (for _array_element_3 _outactors_3
                        (Default|SetEnemyType _array_element_3 _enemytype_2)
                        (Default|SetCursorAnime (Variables|Default|GetStandbyUI) true)))))))))))))

(event Input|KeyboardEvents|A
  (params (Key :type Key%20Structure))
  (bind _standbyui (Variables|Default|GetStandbyUI))
  (bind _standbyui_2 (Variables|Default|GetStandbyUI))
  ;[1 1 1] 右ウィンドウAnd巣を設置操作
  (:Pressed
    (if (not (Variables|/Game/Main/UI/StandbyUI.StandbyUI_C|GetNoInput (Variables|Default|GetStandbyUI)))
      (if (Variables|Default|GetTitleMode)
        (Variables|Default|SetCursorNumber 0)
        (Default|SetCursorNumber (Variables|Default|GetStandbyUI))
        (elif (Variables|Default|GetNestTips)
          (if (Variables|Default|GetNestON)
            (Variables|Default|SetTimeCursorNumber (Variables|Default|GetCursorNumber))
            (bind _result (Math|Integer|DecrementInt (Variables|Default|GetCursorNumber))
              (:%20%20
                (if (< _result 0)
                  (bind _output_get (Variables|Default|SetCursorNumber (- (Variables|Default|GetNestPointNum) 1)))
                  (Default|SetCursorNumber (Variables|Default|GetStandbyUI) _output_get)
                  (else
                    (bind _output_get_2 (Variables|Default|SetCursorNumber _result))
                    (Default|SetCursorNumber (Variables|Default|GetStandbyUI) _output_get_2)))
                (bind _outactors (Actor|GetAllActorsOfClass "/Game/Main/Blueprints/NestPointBP.NestPointBP_C"))
                (for _array_element _outactors
                  (if (== (Variables|Default|GetCursorNumber) (Variables|/Game/Main/Blueprints/NestPointBP.NestPointBP_C|GetPointNumber _array_element))
                    (Default|SetYajirusiVisi _array_element true)
                    (bind _neston (Default|GetNestON _array_element))
                    (Default|SetNestCheck (Variables|Default|GetStandbyUI) _neston)
                    (elif (== (Variables|/Game/Main/Blueprints/NestPointBP.NestPointBP_C|GetPointNumber _array_element) (Variables|Default|GetTimeCursorNumber))
                      (Default|SetYajirusiVisi _array_element false))))))
            (else
              (bind _result_2 (Math|Integer|DecrementInt (Variables|Default|GetCursorNumber))
                (:%20%20
                  (if (< _result_2 0)
                    (bind _output_get_3 (Variables|Default|SetCursorNumber 2))
                    (Default|SetCursorNumber _standbyui _output_get_3)
                    (bind _enemytype (Default|GetEnemyType _standbyui _output_get_3))
                    (bind _outactors_2 (Actor|GetAllActorsOfClass "/Game/Main/UI/UMGActor2DCapture.UMGActor2DCapture_C"))
                    (for _array_element_2 _outactors_2
                      (Default|SetEnemyType _array_element_2 _enemytype)
                      (Default|SetCursorAnime (Variables|Default|GetStandbyUI) false))
                    (else
                      (bind _output_get_4 (Variables|Default|SetCursorNumber _result_2))
                      (Default|SetCursorNumber _standbyui_2 _output_get_4)
                      (bind _enemytype_2 (Default|GetEnemyType _standbyui_2 _output_get_4))
                      (bind _outactors_3 (Actor|GetAllActorsOfClass "/Game/Main/UI/UMGActor2DCapture.UMGActor2DCapture_C"))
                      (for _array_element_3 _outactors_3
                        (Default|SetEnemyType _array_element_3 _enemytype_2)
                        (Default|SetCursorAnime (Variables|Default|GetStandbyUI) false)))))))))))))

(event Input|KeyboardEvents|L
  (params (Key :type Key%20Structure))
  (bind _standbyui (Variables|Default|GetStandbyUI))
  ;[1 1 1] 設置されている巣を消す処理
  (:Pressed
    (if (Variables|Default|GetNestTips)
      (if (not (Variables|Default|GetNestON))
        (bind _nestset (Default|GetNestSet (Variables|Default|GetStandbyUI) (Variables|Default|GetCursorNumber)))
        (if _nestset
          (bind _enemytype (Default|GetEnemyType _standbyui (Variables|Default|GetCursorNumber)))
          (bind _outactors (Actor|GetAllActorsOfClass "/Game/Main/Blueprints/NestPointBP.NestPointBP_C"))
          (for _array_element _outactors
            (Default|SetNestDelete _array_element _enemytype)
            (Default|SetNestSet2 _standbyui false (Variables|Default|GetCursorNumber))
            (Default|SetNestON _array_element false))
          (Default|MinusNestCounter _standbyui))))))

(event Input|KeyboardEvents|W
  (params (Key :type Key%20Structure))
  ;[1 1 1] 左ウィンドウ操作
  (:Pressed
    (if (not (Variables|/Game/Main/UI/StandbyUI.StandbyUI_C|GetNoInput (Variables|Default|GetStandbyUI)))
      (if (not (Variables|Default|GetTitleMode))
        (if (not (Variables|Default|GetNestTips))
          (bind _result (Math|Integer|DecrementInt (Variables|Default|GetCursorNumber))
            (:%20%20
              (if (< _result 0)
                (bind _output_get (Variables|Default|SetCursorNumber 2))
                (Default|SetCursorNumber (Variables|Default|GetStandbyUI) _output_get)
                (else
                  (bind _output_get_2 (Variables|Default|SetCursorNumber _result))
                  (Default|SetCursorNumber (Variables|Default|GetStandbyUI) _output_get_2))))))))))

(event Input|GamepadEvents|GamepadLeftStickRight
  (params (Key :type Key%20Structure))
  (bind _standbyui (Variables|Default|GetStandbyUI))
  (bind _standbyui_2 (Variables|Default|GetStandbyUI))
  ;[1 1 1] 右ウィンドウAnd巣を設置操作
  (:Pressed
    (if (Class|KismetInputLibrary|KeyIsValid Key)
      (if (not (Variables|/Game/Main/UI/StandbyUI.StandbyUI_C|GetNoInput (Variables|Default|GetStandbyUI)))
        (if (Variables|Default|GetTitleMode)
          (bind _output_get (Variables|Default|SetCursorNumber 1))
          (Default|SetCursorNumber (Variables|Default|GetStandbyUI) _output_get)
          (elif (Variables|Default|GetNestTips)
            (if (Variables|Default|GetNestON)
              (Variables|Default|SetTimeCursorNumber (Variables|Default|GetCursorNumber))
              (bind _result (Math|Integer|IncrementInt (Variables|Default|GetCursorNumber))
                (:%20%20
                  (if (> _result (- (Variables|Default|GetNestPointNum) 1))
                    (bind _output_get_2 (Variables|Default|SetCursorNumber 0))
                    (Default|SetCursorNumber (Variables|Default|GetStandbyUI) _output_get_2)
                    (else
                      (bind _output_get_3 (Variables|Default|SetCursorNumber _result))
                      (Default|SetCursorNumber (Variables|Default|GetStandbyUI) _output_get_3)))
                  (bind _outactors (Actor|GetAllActorsOfClass "/Game/Main/Blueprints/NestPointBP.NestPointBP_C"))
                  (for _array_element _outactors
                    (if (== (Variables|Default|GetCursorNumber) (Variables|/Game/Main/Blueprints/NestPointBP.NestPointBP_C|GetPointNumber _array_element))
                      (Default|SetYajirusiVisi _array_element true)
                      (bind _neston (Default|GetNestON _array_element))
                      (Default|SetNestCheck (Variables|Default|GetStandbyUI) _neston)
                      (elif (== (Variables|/Game/Main/Blueprints/NestPointBP.NestPointBP_C|GetPointNumber _array_element) (Variables|Default|GetTimeCursorNumber))
                        (Default|SetYajirusiVisi _array_element false))))))
              (else
                (bind _result_2 (Math|Integer|IncrementInt (Variables|Default|GetCursorNumber))
                  (:%20%20
                    (if (> _result_2 2)
                      (bind _output_get_4 (Variables|Default|SetCursorNumber 0))
                      (Default|SetCursorNumber _standbyui _output_get_4)
                      (bind _enemytype (Default|GetEnemyType _standbyui _output_get_4))
                      (bind _outactors_2 (Actor|GetAllActorsOfClass "/Game/Main/UI/UMGActor2DCapture.UMGActor2DCapture_C"))
                      (for _array_element_2 _outactors_2
                        (Default|SetEnemyType _array_element_2 _enemytype)
                        (Default|SetCursorAnime (Variables|Default|GetStandbyUI) true))
                      (else
                        (bind _output_get_5 (Variables|Default|SetCursorNumber _result_2))
                        (Default|SetCursorNumber _standbyui_2 _output_get_5)
                        (bind _enemytype_2 (Default|GetEnemyType _standbyui_2 _output_get_5))
                        (bind _outactors_3 (Actor|GetAllActorsOfClass "/Game/Main/UI/UMGActor2DCapture.UMGActor2DCapture_C"))
                        (for _array_element_3 _outactors_3
                          (Default|SetEnemyType _array_element_3 _enemytype_2)
                          (Default|SetCursorAnime (Variables|Default|GetStandbyUI) true))))))))))))))

(event Input|KeyboardEvents|S
  (params (Key :type Key%20Structure))
  ;[1 1 1] 左ウィンドウ操作
  (:Pressed
    (if (not (Variables|/Game/Main/UI/StandbyUI.StandbyUI_C|GetNoInput (Variables|Default|GetStandbyUI)))
      (if (not (Variables|Default|GetTitleMode))
        (if (not (Variables|Default|GetNestTips))
          (bind _result (Math|Integer|IncrementInt (Variables|Default|GetCursorNumber))
            (:%20%20
              (if (> _result 2)
                (bind _output_get (Variables|Default|SetCursorNumber 0))
                (Default|SetCursorNumber (Variables|Default|GetStandbyUI) _output_get)
                (else
                  (bind _output_get_2 (Variables|Default|SetCursorNumber _result))
                  (Default|SetCursorNumber (Variables|Default|GetStandbyUI) _output_get_2))))))))))

(event Input|GamepadEvents|GamepadFaceButtonRight
  (params (Key :type Key%20Structure))
  (bind _standbyui (Variables|Default|GetStandbyUI))
  (bind _standbyui_2 (Variables|Default|GetStandbyUI))
  (:Pressed
    (if (not (Variables|Default|GetGameStart))
      (if (Variables|Default|GetNestTips)
        (if (Variables|Default|GetNestON)
          (Variables|Default|SetNestON false)
          (Default|SetNestON (Variables|Default|GetStandbyUI) false)
          ;[1 1 1] 巣の説明召喚
          (bind _output_get (Variables|Default|SetCursorNumber 0))
          (Default|SetNestTips _standbyui_2 true)
          (Variables|Default|SetNestTips true)
          (Default|SetCursorNumber _standbyui_2 _output_get)
          (bind _enemytype (Default|GetEnemyType _standbyui_2 _output_get))
          (bind _outactors (Actor|GetAllActorsOfClass "/Game/Main/UI/UMGActor2DCapture.UMGActor2DCapture_C"))
          (for _array_element _outactors
            (Default|SetEnemyType _array_element _enemytype))
          (else
            (bind _output_get_2 (Variables|Default|SetCursorNumber 0))
            (Default|SetNestTips _standbyui false)
            (Variables|Default|SetNestTips false)
            (Default|SetCursorNumber _standbyui _output_get_2)))))))

(event Input|KeyboardEvents|Enter
  (params (Key :type Key%20Structure))
  (bind _standbyui (Variables|Default|GetStandbyUI))
  (bind _standbyui_2 (Variables|Default|GetStandbyUI))
  (bind _standbyui_3 (Variables|Default|GetStandbyUI))
  (bind _standbyui_4 (Variables|Default|GetStandbyUI))
  (bind _standbyui_5 (Variables|Default|GetStandbyUI))
  (:Pressed
    (if (not (Variables|Default|GetGameStart))
      (if (Variables|Default|GetTitleMode)
        (switch int (Variables|Default|GetCursorNumber)
          (:1
            (Variables|Default|SetTitleMode false)
            (Variables|Default|SetCursorNumber 0)
            (Default|SetTitleMode _standbyui_4 false)
            (Default|SetCursorNumber _standbyui_4)))
        (elif (Variables|Default|GetNestTips)
          (if (Variables|Default|GetNestON)
            ;[1 1 1] 巣を設置
            (bind _outactors (Actor|GetAllActorsOfClass "/Game/Main/Blueprints/NestPointBP.NestPointBP_C"))
            (for _array_element _outactors
              (if (== (Variables|Default|GetCursorNumber) (Variables|/Game/Main/Blueprints/NestPointBP.NestPointBP_C|GetPointNumber _array_element))
                (bind (_ischenge _nesttype1) (Default|SetNestCreate _array_element (Variables|Default|GetNestType)))
                (if _ischenge
                  (Default|SetNestSetAllReset _standbyui_5 _nesttype1)
                  (else
                    (Default|AddNestCounter _standbyui_5)))
                (Default|SetNestSet _standbyui_5 true)
                (Default|SetYajirusiVisi _array_element false)))
            (Variables|Default|SetNestON false)
            (Default|SetNestON (Variables|Default|GetStandbyUI) false)
            ;[1 1 1] 巣の説明召喚
            (bind _output_get (Variables|Default|SetCursorNumber 0 :!label _label))
            (Default|SetNestTips _standbyui_3 true)
            (Variables|Default|SetNestTips true)
            (Default|SetCursorNumber _standbyui_3 _output_get)
            (bind _enemytype (Default|GetEnemyType _standbyui_3 _output_get))
            (bind _outactors_2 (Actor|GetAllActorsOfClass "/Game/Main/UI/UMGActor2DCapture.UMGActor2DCapture_C"))
            (for _array_element_2 _outactors_2
              (Default|SetEnemyType _array_element_2 _enemytype))
            (else
              (bind _nestset (Default|GetNestSet (Variables|Default|GetStandbyUI) (Variables|Default|GetCursorNumber)))
              ;[1 1 1] 巣の設置画面へ
              (if (not _nestset)
                (Default|SetNestType _standbyui_2 (Variables|Default|GetCursorNumber))
                (bind _output_get_2 (Variables|Default|SetCursorNumber 0))
                (Default|SetNestON _standbyui_2 true _output_get_2)
                (Variables|Default|SetNestON true)
                (Default|SetCursorNumber _standbyui_2 _output_get_2)
                (bind _newparam (Default|GetNestType _standbyui_2))
                (Variables|Default|SetNestType _newparam)
                (bind _outactors_3 (Actor|GetAllActorsOfClass "/Game/Main/Blueprints/NestPointBP.NestPointBP_C"))
                (for _array_element_3 _outactors_3
                  (if (== (Variables|Default|GetCursorNumber) (Variables|/Game/Main/Blueprints/NestPointBP.NestPointBP_C|GetPointNumber _array_element_3))
                    (Default|SetYajirusiVisi _array_element_3 true)
                    (bind _neston (Default|GetNestON _array_element_3))
                    (if _neston
                      (Default|SetNestCheck (Variables|Default|GetStandbyUI) true)))))))
          (else
            (switch int (Variables|Default|GetCursorNumber) ; 左のウィンドウがアクティブの時
              (:0
                (if (> (Variables|/Game/Main/UI/StandbyUI.StandbyUI_C|GetNestCounter (Variables|Default|GetStandbyUI)) 0)
                  (bind _output_get_3 (Variables|Default|SetGameStart true))
                  (Default|SetGameStart (Variables|Default|GetStandbyUI) _output_get_3)))
              (:1
                (goto _label))
              (:2
                (bind _output_get_4 (Variables|Default|SetTitleMode true))
                (bind _output_get_5 (Variables|Default|SetCursorNumber 1))
                (Default|SetTitleMode _standbyui _output_get_4)
                (Default|SetCursorNumber _standbyui _output_get_5)))))))))

(event Input|GamepadEvents|GamepadFaceButtonBottom
  (params (Key :type Key%20Structure))
  (bind _standbyui (Variables|Default|GetStandbyUI))
  (bind _standbyui_2 (Variables|Default|GetStandbyUI))
  (bind _standbyui_3 (Variables|Default|GetStandbyUI))
  (bind _standbyui_4 (Variables|Default|GetStandbyUI))
  (bind _standbyui_5 (Variables|Default|GetStandbyUI))
  (:Pressed
    (if (not (Variables|Default|GetGameStart))
      (if (Variables|Default|GetTitleMode)
        (switch int (Variables|Default|GetCursorNumber)
          (:1
            (Variables|Default|SetTitleMode false)
            (Variables|Default|SetCursorNumber 0)
            (Default|SetTitleMode _standbyui_4 false)
            (Default|SetCursorNumber _standbyui_4)))
        (elif (Variables|Default|GetNestTips)
          (if (Variables|Default|GetNestON)
            ;[1 1 1] 巣を設置
            (bind _outactors (Actor|GetAllActorsOfClass "/Game/Main/Blueprints/NestPointBP.NestPointBP_C"))
            (for _array_element _outactors
              (if (== (Variables|Default|GetCursorNumber) (Variables|/Game/Main/Blueprints/NestPointBP.NestPointBP_C|GetPointNumber _array_element))
                (bind (_ischenge _nesttype1) (Default|SetNestCreate _array_element (Variables|Default|GetNestType)))
                (if _ischenge
                  (Default|SetNestSetAllReset _standbyui_5 _nesttype1)
                  (else
                    (Default|AddNestCounter _standbyui_5)))
                (Default|SetNestSet _standbyui_5 true)
                (Default|SetYajirusiVisi _array_element false)))
            (Variables|Default|SetNestON false)
            (Default|SetNestON (Variables|Default|GetStandbyUI) false)
            ;[1 1 1] 巣の説明召喚
            (bind _output_get (Variables|Default|SetCursorNumber 0 :!label _label))
            (Default|SetNestTips _standbyui_3 true)
            (Variables|Default|SetNestTips true)
            (Default|SetCursorNumber _standbyui_3 _output_get)
            (bind _enemytype (Default|GetEnemyType _standbyui_3 _output_get))
            (bind _outactors_2 (Actor|GetAllActorsOfClass "/Game/Main/UI/UMGActor2DCapture.UMGActor2DCapture_C"))
            (for _array_element_2 _outactors_2
              (Default|SetEnemyType _array_element_2 _enemytype))
            (else
              (bind _nestset (Default|GetNestSet (Variables|Default|GetStandbyUI) (Variables|Default|GetCursorNumber)))
              ;[1 1 1] 巣の設置画面へ
              (if (not _nestset)
                (Default|SetNestType _standbyui_2 (Variables|Default|GetCursorNumber))
                (bind _output_get_2 (Variables|Default|SetCursorNumber 0))
                (Default|SetNestON _standbyui_2 true _output_get_2)
                (Variables|Default|SetNestON true)
                (Default|SetCursorNumber _standbyui_2 _output_get_2)
                (bind _newparam (Default|GetNestType _standbyui_2))
                (Variables|Default|SetNestType _newparam)
                (bind _outactors_3 (Actor|GetAllActorsOfClass "/Game/Main/Blueprints/NestPointBP.NestPointBP_C"))
                (for _array_element_3 _outactors_3
                  (if (== (Variables|Default|GetCursorNumber) (Variables|/Game/Main/Blueprints/NestPointBP.NestPointBP_C|GetPointNumber _array_element_3))
                    (Default|SetYajirusiVisi _array_element_3 true)
                    (bind _neston (Default|GetNestON _array_element_3))
                    (if _neston
                      (Default|SetNestCheck (Variables|Default|GetStandbyUI) true)))))))
          (else
            (switch int (Variables|Default|GetCursorNumber) ; 左のウィンドウがアクティブの時
              (:0
                (if (> (Variables|/Game/Main/UI/StandbyUI.StandbyUI_C|GetNestCounter (Variables|Default|GetStandbyUI)) 0)
                  (bind _output_get_3 (Variables|Default|SetGameStart true))
                  (Default|SetGameStart (Variables|Default|GetStandbyUI) _output_get_3)))
              (:1
                (goto _label))
              (:2
                (bind _output_get_4 (Variables|Default|SetTitleMode true))
                (bind _output_get_5 (Variables|Default|SetCursorNumber 1))
                (Default|SetTitleMode _standbyui _output_get_4)
                (Default|SetCursorNumber _standbyui _output_get_5)))))))))

(event Input|KeyboardEvents|Backspace
  (params (Key :type Key%20Structure))
  (bind _standbyui (Variables|Default|GetStandbyUI))
  (bind _standbyui_2 (Variables|Default|GetStandbyUI))
  (:Pressed
    (if (not (Variables|Default|GetGameStart))
      (if (Variables|Default|GetNestTips)
        (if (Variables|Default|GetNestON)
          (Variables|Default|SetNestON false)
          (Default|SetNestON (Variables|Default|GetStandbyUI) false)
          ;[1 1 1] 巣の説明召喚
          (bind _output_get (Variables|Default|SetCursorNumber 0))
          (Default|SetNestTips _standbyui_2 true)
          (Variables|Default|SetNestTips true)
          (Default|SetCursorNumber _standbyui_2 _output_get)
          (bind _enemytype (Default|GetEnemyType _standbyui_2 _output_get))
          (bind _outactors (Actor|GetAllActorsOfClass "/Game/Main/UI/UMGActor2DCapture.UMGActor2DCapture_C"))
          (for _array_element _outactors
            (Default|SetEnemyType _array_element _enemytype))
          (else
            (bind _output_get_2 (Variables|Default|SetCursorNumber 0))
            (Default|SetNestTips _standbyui false)
            (Variables|Default|SetNestTips false)
            (Default|SetCursorNumber _standbyui _output_get_2)))))))

(event Input|GamepadEvents|GamepadFaceButtonLeft
  (params (Key :type Key%20Structure))
  (bind _standbyui (Variables|Default|GetStandbyUI))
  ;[1 1 1] 設置されている巣を消す処理
  (:Pressed
    (if (Variables|Default|GetNestTips)
      (if (not (Variables|Default|GetNestON))
        (bind _nestset (Default|GetNestSet (Variables|Default|GetStandbyUI) (Variables|Default|GetCursorNumber)))
        (if _nestset
          (bind _enemytype (Default|GetEnemyType _standbyui (Variables|Default|GetCursorNumber)))
          (bind _outactors (Actor|GetAllActorsOfClass "/Game/Main/Blueprints/NestPointBP.NestPointBP_C"))
          (for _array_element _outactors
            (Default|SetNestDelete _array_element _enemytype)
            (Default|SetNestSet2 _standbyui false (Variables|Default|GetCursorNumber))
            (Default|SetNestON _array_element false))
          (Default|MinusNestCounter _standbyui))))))

(fn ConstructionScript)

(fn SetNestPointCount
  (bind _result (Math|Integer|IncrementInt (Variables|Default|GetNestPointNum))
    (:%20%20
      (Variables|Default|SetNestPointNum _result))))

(fn SetDestroy
  (Variables|Default|SetbAutoDestroyWhenFinished true))