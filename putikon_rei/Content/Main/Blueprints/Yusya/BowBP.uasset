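; BowBP is a hero's bow projectile that flies to a target position and damages enemies it hits.
; BeginPlay tags the mesh as a bullet and faces it at the target, then Tick moves it a fixed, frame-rate-dependent step.
; Sphere overlap with an enemy-tagged component calls DamageEvent and spawns a damage effect.
; Hits, X/Y arrival and EndEmitter hide the mesh and set AutoDestroyWhenFinished.
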(event OnComponentBeginOverlap(AttackCollision)
  (params (OverlappedComponent :type Primitive%20Component%20Object%20Reference) (OtherActor :type Actor%20Object%20Reference) (OtherComp :type Primitive%20Component%20Object%20Reference) (OtherBodyIndex :type Integer) (bFromSweep :type Boolean) (SweepResult :type Hit%20Result%20Structure%20%28by%20ref%29)))

(event OnComponentBeginOverlap(Sphere)
  (params (OverlappedComponent :type Primitive%20Component%20Object%20Reference) (OtherActor :type Actor%20Object%20Reference) (OtherComp :type Primitive%20Component%20Object%20Reference) (OtherBodyIndex :type Integer) (bFromSweep :type Boolean) (SweepResult :type Hit%20Result%20Structure%20%28by%20ref%29))
  (bind _asglobal_instance (Utilities|Casting|CastToGlobalInstance (Game|GetGameInstance)))
  (if (Components|ComponentHasTag OtherComp (Variables|/Game/Main/GlobalInstance.GlobalInstance_C|GetCollisionEnemyTag _asglobal_instance))
    (bind _asenemy_oyaclass (Utilities|Casting|CastToEnemyOyaclass OtherActor))
    (Default|DamageEvent _asenemy_oyaclass (Variables|Default|GetStr) (Variables|Default|GetNumber))
    (Niagara|SpawnSystematLocation "/Game/Main/particle/niagara/Hit/Damege/DamegeSystem.DamegeSystem" (Transformation|GetWorldLocation (Variables|Default|GetStaticMesh)))
    (Rendering|SetVisibility (Variables|Default|GetStaticMesh) false false)
    (Variables|Default|SetbAutoDestroyWhenFinished true)))

(event EventBeginPlay
  (bind _targetpositiom (Variables|Default|GetTargetPositiom))
  (bind _staticmesh (Variables|Default|GetStaticMesh))
  (bind _returnvalue (Transformation|GetWorldLocation _staticmesh))
  (bind _returnvalue_2 (Math|Rotator|FindLookatRotation _returnvalue _targetpositiom))
  (bind _output_get (Variables|Default|SetMoveSpeed 6e+01))
  (Variables|Default|SetHitLength _output_get)
  (bind _asglobal_instance (Utilities|Casting|CastToGlobalInstance (Game|GetGameInstance)))
  (Utilities|Array|SetArrayElem (Variables|/Script/Engine.ActorComponent|GetComponentTags (Variables|Default|GetStaticMesh)) 0 (Variables|/Game/Main/GlobalInstance.GlobalInstance_C|GetCollisionBulletTag _asglobal_instance) true)
  (Transformation|SetWorldRotation (Variables|Default|GetStaticMesh) (Math|Rotator|MakeRotator (.roll _returnvalue_2) (.pitch _returnvalue_2) (+ (.yaw _returnvalue_2) 1.8e+02)) false false))

(event Collision|EventActorBeginOverlap
  (params (OtherActor :type Actor%20Object%20Reference)))

(event EventTick
  (params (DeltaSeconds :type Float%20%28single-precision%29))
  (bind _targetpositiom (Variables|Default|GetTargetPositiom))
  (if (Rendering|IsVisible (Variables|Default|GetStaticMesh))
    (Utilities|FlowControl|Sequence
      (:then_0
        (bind _output_get (Variables|Default|SetStackPosition (- (Variables|Default|GetTargetPositiom) (Transformation|GetWorldLocation (Variables|Default|GetStaticMesh)))))
        (Transformation|SetWorldLocation (Variables|Default|GetStaticMesh) (+ (* (Math|Vector|Normalize _output_get) (Variables|Default|GetMoveSpeed)) (Transformation|GetWorldLocation (Variables|Default|GetStaticMesh))) false false))
      (:then_1
        ;[1 1 1] ターゲットの位置に着いているか判定
        (if (>= (+ (.x _targetpositiom) (Variables|Default|GetHitLength)) (.x (Transformation|GetWorldLocation (Variables|Default|GetStaticMesh))))
          (if (<= (- (.x _targetpositiom) (Variables|Default|GetHitLength)) (.x (Transformation|GetWorldLocation (Variables|Default|GetStaticMesh))))
            (if (>= (+ (.y _targetpositiom) (Variables|Default|GetHitLength)) (.y (Transformation|GetWorldLocation (Variables|Default|GetStaticMesh))))
              (if (<= (- (.y _targetpositiom) (Variables|Default|GetHitLength)) (.y (Transformation|GetWorldLocation (Variables|Default|GetStaticMesh))))
                (Rendering|SetVisibility (Variables|Default|GetStaticMesh) false false)
                (Variables|Default|SetbAutoDestroyWhenFinished true)))))))))

(event EventEndEmitter
  (Niagara|SpawnSystematLocation "/Game/Main/particle/niagara/Hit/Damege/DamegeSystem.DamegeSystem" (Transformation|GetWorldLocation (Variables|Default|GetStaticMesh)))
  (Rendering|SetVisibility (Variables|Default|GetStaticMesh) false false)
  (Variables|Default|SetbAutoDestroyWhenFinished true))

(fn ConstructionScript
  (|CallParentFunction))