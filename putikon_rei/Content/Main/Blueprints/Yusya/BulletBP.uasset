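; Projectile for a Yusya (hero) that flies a Niagara effect toward a stored target position and damages enemies.
; Each Tick moves the effect a fixed step, not scaled by delta time, and interpolates its yaw toward the target.
; AttackCollision overlaps with enemy-tagged components call DamageEvent on EnemyOyaclass with strength and Yusya number.
; A hit, or arrival within one step of the target in X/Y, sets AutoDestroyWhenFinished.
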(event OnComponentBeginOverlap(AttackCollision)
  (params (OverlappedComponent :type Primitive%20Component%20Object%20Reference) (OtherActor :type Actor%20Object%20Reference) (OtherComp :type Primitive%20Component%20Object%20Reference) (OtherBodyIndex :type Integer) (bFromSweep :type Boolean) (SweepResult :type Hit%20Result%20Structure%20%28by%20ref%29))
  (bind _asglobal_instance (Utilities|Casting|CastToGlobalInstance (Game|GetGameInstance)))
  (if (Components|ComponentHasTag OtherComp (Variables|/Game/Main/GlobalInstance.GlobalInstance_C|GetCollisionEnemyTag _asglobal_instance))
    (bind _asenemy_oyaclass (Utilities|Casting|CastToEnemyOyaclass OtherActor))
    (Default|DamageEvent _asenemy_oyaclass (Variables|Default|GetStr) (Variables|Default|GetNumber))
    (Variables|Default|SetbAutoDestroyWhenFinished true)))

(event EventBeginPlay
  (bind _output_get (Variables|Default|SetMoveSpeed 1e+02))
  (Variables|Default|SetHitLength _output_get))

(event Collision|EventActorBeginOverlap
  (params (OtherActor :type Actor%20Object%20Reference)))

(event EventTick
  (params (DeltaSeconds :type Float%20%28single-precision%29))
  (bind _targetpositiom (Variables|Default|GetTargetPositiom))
  (bind _niagara (Variables|Default|GetNiagara))
  (bind _niagara_2 (Variables|Default|GetNiagara))
  (bind _returnvalue (Transformation|GetWorldRotation _niagara_2))
  (bind _returnvalue_2 (Transformation|GetWorldLocation _niagara))
  (Utilities|FlowControl|Sequence
    (:then_0
      (bind _output_get (Variables|Default|SetStackPosition (- (Variables|Default|GetTargetPositiom) (Transformation|GetWorldLocation (Variables|Default|GetNiagara)))))
      (Transformation|SetWorldLocation _niagara (+ (* (Math|Vector|Normalize _output_get) (Variables|Default|GetMoveSpeed)) _returnvalue_2) false false)
      ;[1 1 1] 徐々にターゲットの方に回転させる
      (Transformation|SetWorldRotation (Variables|Default|GetNiagara) (CallFunction|RInterptoQuaternionFunction (Transformation|GetWorldRotation (Variables|Default|GetNiagara)) (Math|Rotator|MakeRotator (.roll _returnvalue) (.pitch _returnvalue) (+ (.yaw (Math|Rotator|FindLookatRotation _returnvalue_2 (Variables|Default|GetTargetPositiom))) -9e+01)) (Utilities|Time|GetWorldDeltaSeconds) 5e+02) false false))
    (:then_1
      ;[1 1 1] ターゲットの位置に着いているか判定
      (if (>= (+ (.x _targetpositiom) (Variables|Default|GetHitLength)) (.x (Transformation|GetWorldLocation (Variables|Default|GetNiagara))))
        (if (<= (- (.x _targetpositiom) (Variables|Default|GetHitLength)) (.x (Transformation|GetWorldLocation (Variables|Default|GetNiagara))))
          (if (>= (+ (.y _targetpositiom) (Variables|Default|GetHitLength)) (.y (Transformation|GetWorldLocation (Variables|Default|GetNiagara))))
            (if (<= (- (.y _targetpositiom) (Variables|Default|GetHitLength)) (.y (Transformation|GetWorldLocation (Variables|Default|GetNiagara))))
              (Variables|Default|SetbAutoDestroyWhenFinished true))))))))

(fn ConstructionScript)