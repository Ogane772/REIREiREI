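; FireBP is an actor, under the Yusya blueprints, that sends a Niagara effect travelling toward a target position.
; Each Tick shifts the effect a fixed step along the direction from the skeletal mesh to the target, so speed depends on frame rate.
; It also interpolates the effect's yaw toward the target through a quaternion helper, with a quarter-turn offset, keeping pitch and roll.
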(event EventBeginPlay)

(event Collision|EventActorBeginOverlap
  (params (OtherActor :type Actor%20Object%20Reference)))

(event EventTick
  (params (DeltaSeconds :type Float%20%28single-precision%29))
  (bind _niagara (Variables|Default|GetNiagara))
  (bind _niagara_2 (Variables|Default|GetNiagara))
  (bind _returnvalue (Transformation|GetWorldRotation _niagara))
  (bind _returnvalue_2 (Transformation|GetWorldLocation _niagara_2))
  (Utilities|FlowControl|Sequence
    (:then_0
      (bind _output_get (Variables|Default|SetStackPosition (- (Variables|Default|GetTargetPositiom) (Transformation|GetWorldLocation (Variables|Vehicle|GetSkeletalMesh)))))
      (Transformation|SetWorldLocation _niagara_2 (+ (* (Math|Vector|Normalize _output_get) 1e+01) _returnvalue_2) false false)
      ;[1 1 1] 徐々にターゲットの方に回転させる
      (Transformation|SetWorldRotation (Variables|Default|GetNiagara) (CallFunction|RInterptoQuaternion (Transformation|GetWorldRotation (Variables|Default|GetNiagara)) (Math|Rotator|MakeRotator (.roll _returnvalue) (.pitch _returnvalue) (+ (.yaw (Math|Rotator|FindLookatRotation _returnvalue_2 (Variables|Default|GetTargetPositiom))) -9e+01)) (Utilities|Time|GetWorldDeltaSeconds) 5e+02) false false))))

(fn ConstructionScript)