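; Hero unit (Yusya08), a ranged magician variant of its parent Yusya class that targets a castle, nest or enemy according to its order.
; BeginPlay sets stats, snipe mode and target position; Tick runs the parent logic and drives Yusya03Anime for walking, attacking and death.
; In attack mode it turns toward the enemy or revenge target, and tagged AttackCollision overlaps trigger timed attacks that spawn a magic effect and delayed bullet.
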(event OnComponentBeginOverlap(AttackCollision)
  (params (OverlappedComponent :type Primitive%20Component%20Object%20Reference) (OtherActor :type Actor%20Object%20Reference) (OtherComp :type Primitive%20Component%20Object%20Reference) (OtherBodyIndex :type Integer) (bFromSweep :type Boolean) (SweepResult :type Hit%20Result%20Structure%20%28by%20ref%29))
  ;[1 1 1] 攻撃中
  (if (Components|ComponentHasTag OtherComp (Variables|/Game/Main/GlobalInstance.GlobalInstance_C|GetCollisionEnemyTag (.AsGlobal%20Instance (Utilities|Casting|CastToGlobalInstance (Game|GetGameInstance)))))
    (Variables|Default|SetAttackStart true)
    (elif (Components|ComponentHasTag OtherComp (Variables|/Game/Main/GlobalInstance.GlobalInstance_C|GetCollisionHaniAttackTag (.AsGlobal%20Instance (Utilities|Casting|CastToGlobalInstance (Game|GetGameInstance)))))
      (Variables|Default|SetAttackStart true))))

(event OnComponentEndOverlap(AttackCollision)
  (params (OverlappedComponent :type Primitive%20Component%20Object%20Reference) (OtherActor :type Actor%20Object%20Reference) (OtherComp :type Primitive%20Component%20Object%20Reference) (OtherBodyIndex :type Integer))
  ;[1 1 1] 攻撃中
  (if (Components|ComponentHasTag OtherComp (Variables|/Game/Main/GlobalInstance.GlobalInstance_C|GetCollisionEnemyTag (.AsGlobal%20Instance (Utilities|Casting|CastToGlobalInstance (Game|GetGameInstance)))))
    (Variables|Default|SetAttackStart false :!label _label)
    (Collision|SetCollisionEnabled (Variables|Default|GetAttackCollision) "NoCollision")
    (elif (Components|ComponentHasTag OtherComp (Variables|/Game/Main/GlobalInstance.GlobalInstance_C|GetCollisionHaniAttackTag (.AsGlobal%20Instance (Utilities|Casting|CastToGlobalInstance (Game|GetGameInstance)))))
      (goto _label))))

(event EventBeginPlay
  ;[1 1 1] BeginPlay
  (Variables|Default|SetSnipeMode true)
  (|CallParentFunction)
  (bind _asyusya_03anime (Utilities|Casting|CastToYusya03Anime (Components|SkeletalMesh|GetAnimInstance (Variables|Default|Getbody))))
  (Variables|Default|SetAnime _asyusya_03anime)
  (Collision|SetCollisionEnabled (Variables|Default|GetSnipeCollision) "NoCollision")
  (Variables|Default|SetMoveSpeed 1e+01)
  (bind _output_get (Variables|Default|SetHP 4e+01))
  (Variables|Default|SetMAXHP _output_get)
  (Collision|SetCollisionEnabled (Variables|Default|GetAttackCollision) "NoCollision")
  (switch Utilities|FlowControl|Switch|SwitchonYusyaOrderEnum (Variables|Default|GetYusyaOrder)
    (:NewEnumerator0
      (bind _outactors (Actor|GetAllActorsOfClass "/Game/Main/Blueprints/PlayerCastle.PlayerCastle_C"))
      (for _array_element _outactors
        (bind _targetpoint (Default|GetCastleTargetPoint _array_element))
        (Variables|Default|SetTargetPosition _targetpoint)))
    (:NewEnumerator1
      (bind _nestpotision (CallFunction|GetNestPotision))
      (Variables|Default|SetTargetPosition _nestpotision))
    (:NewEnumerator2
      (bind _enemypotision (CallFunction|GetEnemyPotision))
      (Variables|Default|SetTargetPosition _enemypotision))))

(event Collision|EventActorBeginOverlap
  (params (OtherActor :type Actor%20Object%20Reference))
  (|CallParentFunction OtherActor) ; This node is disabled and will not be called.\nDrag off pins to build functionality.
)

(event EventTick
  (params (DeltaSeconds :type Float%20%28single-precision%29))
  (bind _rightweapon (Variables|Default|GetRightWeapon))
  (bind _returnvalue (Transformation|GetWorldLocation _rightweapon))
  (if (Variables|Default|GetIsDeath)
    ;[1 1 1] 死亡時の処理
    (Utilities|FlowControl|Sequence
      (:then_0
        (Utilities|FlowControl|DoOnce false
          (:Completed
            (Default|Death (Variables|Default|GetAnime)))))
      (:then_1
        (if (Variables|/Game/Main/Blueprints/Yusya/Yusya03Anime.Yusya03Anime_C|GetIsDeath (Variables|Default|GetAnime))
          (Variables|Default|SetbAutoDestroyWhenFinished true)))
      (:then_2
        (|CameraMove_2_2_2_2))
      (:then_3
        (|HP＿WARIAI_2_2_2_2)))
    (else
      (|CallParentFunction DeltaSeconds)
      (if (not (Variables|Default|GetAttackMode))
        (Utilities|FlowControl|Sequence
          (:then_0
            (Variables|/Game/Main/Blueprints/Yusya/Yusya03Anime.Yusya03Anime_C|SetIsWalk (Variables|Default|GetAnime) (Variables|Default|GetIsWalk))
            (Collision|SetCollisionEnabled (Variables|Default|GetAttackCollision) "NoCollision"))
          (:then_1
            ;[1 1 1] 攻撃モーションの当たり判定更新
            (if (not (Variables|/Game/Main/Blueprints/Yusya/Yusya03Anime.Yusya03Anime_C|GetAttackOn (Variables|Default|GetAnime))) :!label _label
              (Utilities|FlowControl|Delay 0.5) ; 攻撃でモンスターを倒した後の待機時間
              (Variables|Default|SetNoWalk false))))
        (else
          (Collision|SetCollisionEnabled (Variables|Default|GetAttackCollision) "QueryOnly")
          (Utilities|FlowControl|Sequence
            (:then_0
              (if (Variables|Default|GetRevengeOn)
                (CallFunction|Rotate (Variables|Default|GetRevengeEnemyPosition) 2.5e+02)
                (else
                  (CallFunction|Rotate (Variables|Default|GetEnemyPosition) 2.5e+02))))
            (:then_1
              ;[1 1 1] 攻撃モーション＆攻撃時間間隔
              (if (Variables|Default|GetAttackStart)
                (Utilities|FlowControl|DoOnce false :!label _label_2
                  (:Completed
                    (Default|Attack (Variables|Default|GetAnime))
                    (Niagara|SpawnSystematLocation "/Game/Main/particle/niagara/Monster/Monstar_attack/Magician/MagicianAttack_2.MagicianAttack_2" _returnvalue)
                    (Utilities|FlowControl|Delay 1.0)
                    (Game|SpawnActorfromClass "/Game/Main/Blueprints/Yusya/BulletBP.BulletBP_C" (Math|Conversions|ToTransform(Vector) _returnvalue) "Undefined" 0 (Variables|Default|GetTargetPosition) 1.0 (Variables|Default|GetYusyaMyNumber) 0)
                    (Collision|SetCollisionEnabled (Variables|Default|GetAttackCollision) "NoCollision")))))
            (:then_2
              (Utilities|FlowControl|Delay 2.0)
              (goto _label_2 Reset))
            (:then_3
              (goto _label))
            (:then_4
              ;[1 1 1] 攻撃中は歩きモーションをしない
              (Variables|/Game/Main/Blueprints/Yusya/Yusya03Anime.Yusya03Anime_C|SetIsWalk (Variables|Default|GetAnime) false))))))))

(fn ConstructionScript
  (|CallParentFunction))