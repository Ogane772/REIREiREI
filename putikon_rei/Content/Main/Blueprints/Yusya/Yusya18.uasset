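; Hero character Blueprint (Yusya18) that walks, turns toward enemies or revenge targets and deals melee damage.
; In attack mode, Tick rotates it and, once AttackCollision detects a tagged target, triggers timed attacks on the Yusya04Anime instance.
; The animation's AttackOn flag toggles the Capsule0 hitbox, which damages EnemyOyaclass actors by Str.
; On death it plays the death animation, spawns a vortex effect and keeps the camera-facing HP bar updated.
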(event OnComponentBeginOverlap(Capsule_0)
  (params (OverlappedComponent :type Primitive%20Component%20Object%20Reference) (OtherActor :type Actor%20Object%20Reference) (OtherComp :type Primitive%20Component%20Object%20Reference) (OtherBodyIndex :type Integer) (bFromSweep :type Boolean) (SweepResult :type Hit%20Result%20Structure%20%28by%20ref%29))
  ;[1 1 1] 攻撃の当たり判定
  (if (Variables|/Game/Main/Blueprints/Yusya/Yusya04Anime.Yusya04Anime_C|GetAttackOn (Variables|Default|GetAnime))
    (if (Utilities|ClassIsChildOf (Utilities|GetClass OtherActor) "/Game/Main/Blueprints/Enemy/EnemyOyaclass.EnemyOyaclass_C")
      (bind _asenemy_oyaclass (Utilities|Casting|CastToEnemyOyaclass OtherActor :!label _label))
      (Default|DamageEvent _asenemy_oyaclass (Variables|Default|GetStr) (Variables|Default|GetYusyaMyNumber))
      (Variables|Default|SetNoWalk true))
    (else
      (bind _asglobal_instance (Utilities|Casting|CastToGlobalInstance (Game|GetGameInstance)))
      (if (Components|ComponentHasTag OtherComp (Variables|/Game/Main/GlobalInstance.GlobalInstance_C|GetCollisionEnemyTag _asglobal_instance))
        (goto _label)))))

(event OnComponentBeginOverlap(AttackCollision)
  (params (OverlappedComponent :type Primitive%20Component%20Object%20Reference) (OtherActor :type Actor%20Object%20Reference) (OtherComp :type Primitive%20Component%20Object%20Reference) (OtherBodyIndex :type Integer) (bFromSweep :type Boolean) (SweepResult :type Hit%20Result%20Structure%20%28by%20ref%29))
  ;[1 1 1] 攻撃中
  (if (Components|ComponentHasTag OtherComp (Variables|/Game/Main/GlobalInstance.GlobalInstance_C|GetCollisionEnemyTag (.AsGlobal%20Instance (Utilities|Casting|CastToGlobalInstance (Game|GetGameInstance)))))
    (Variables|Default|SetAttackStart true)
    (elif (Components|ComponentHasTag OtherComp (Variables|/Game/Main/GlobalInstance.GlobalInstance_C|GetCollisionHaniAttackTag (.AsGlobal%20Instance (Utilities|Casting|CastToGlobalInstance (Game|GetGameInstance)))))
      (Variables|Default|SetAttackStart true))))

(event OnComponentEndOverlap(AttackCollision)
  (params (OverlappedComponent :type Primitive%20Component%20Object%20Reference) (OtherActor :type Actor%20Object%20Reference) (OtherComp :type Primitive%20Component%20Object%20Reference) (OtherBodyIndex :type Integer))
  ;[1 1 1] 攻撃中
  (if (Components|ComponentHasTag OtherComp (Variables|/Game/Main/GlobalInstance.GlobalInstance_C|GetCollisionEnemyTag (.AsGlobal%20Instance (Utilities|Casting|CastToGlobalInstance (Game|GetGameInstance)))))
    (Variables|Default|SetAttackStart false :!label _label)
    (Collision|SetCollisionEnabled (Variables|Default|GetAttackCollision) "NoCollision")
    (elif (Components|ComponentHasTag OtherComp (Variables|/Game/Main/GlobalInstance.GlobalInstance_C|GetCollisionHaniAttackTag (.AsGlobal%20Instance (Utilities|Casting|CastToGlobalInstance (Game|GetGameInstance)))))
      (goto _label))))

(event EventBeginPlay
  ;[1 1 1] BeginPlay
  (|CallParentFunction)
  (bind _asyusya_04anime (Utilities|Casting|CastToYusya04Anime (Components|SkeletalMesh|GetAnimInstance (Variables|Default|Getbody))))
  (Variables|Default|SetAnime _asyusya_04anime)
  (Collision|SetCollisionEnabled (Variables|Default|GetSnipeCollision) "NoCollision")
  (CallFunction|SetCollision false (Variables|Default|GetCapsule_0))
  (Collision|SetCollisionEnabled (Variables|Default|GetAttackCollision) "NoCollision")
  (bind _asglobal_instance (Utilities|Casting|CastToGlobalInstance (Game|GetGameInstance))))

(event Collision|EventActorBeginOverlap
  (params (OtherActor :type Actor%20Object%20Reference))
  (|CallParentFunction OtherActor) ; This node is disabled and will not be called.\nDrag off pins to build functionality.
)

(event EventTick
  (params (DeltaSeconds :type Float%20%28single-precision%29))
  (Development|PrintString (Utilities|String|ToString(Float) (Variables|Default|GetMoveSpeed)) true true "(R=0.075107,G=0.056700,B=1.000000,A=1.000000)" 0.0)
  (if (Variables|Default|GetIsDeath)
    ;[1 1 1] 死亡時の処理
    (Utilities|FlowControl|Sequence
      (:then_0
        (Utilities|FlowControl|DoOnce false
          (:Completed
            (Default|Death (Variables|Default|GetAnime)))))
      (:then_1
        (if (Variables|/Game/Main/Blueprints/Yusya/Yusya04Anime.Yusya04Anime_C|GetIsDeath (Variables|Default|GetAnime))
          (Niagara|SpawnSystematLocation "/Game/Main/particle/niagara/Vortex/VortexSystem_3.VortexSystem_3" (Transformation|GetWorldLocation (Variables|Default|Getbody)))
          (Variables|Default|SetbAutoDestroyWhenFinished true)))
      (:then_2
        (|CameraMove_2_2_2_2))
      (:then_3
        (|HP＿WARIAI_2_2_2_2)))
    (else
      (|CallParentFunction DeltaSeconds)
      (if (not (Variables|Default|GetAttackMode))
        (Utilities|FlowControl|Sequence
          (:then_0
            (Variables|/Game/Main/Blueprints/Yusya/Yusya04Anime.Yusya04Anime_C|SetIsWalk (Variables|Default|GetAnime) (Variables|Default|GetIsWalk))
            (Collision|SetCollisionEnabled (Variables|Default|GetAttackCollision) "NoCollision"))
          (:then_1
            ;[1 1 1] 攻撃モーションの当たり判定更新
            (if (Variables|/Game/Main/Blueprints/Yusya/Yusya04Anime.Yusya04Anime_C|GetAttackOn (Variables|Default|GetAnime)) :!label _label
              (CallFunction|SetCollision true (Variables|Default|GetCapsule_0))
              (else
                (CallFunction|SetCollision false (Variables|Default|GetCapsule_0))
                (Utilities|FlowControl|Delay 0.5) ; 攻撃でモンスターを倒した後の待機時間
                (Variables|Default|SetNoWalk false)))))
        (else
          (Collision|SetCollisionEnabled (Variables|Default|GetAttackCollision) "QueryOnly")
          (Utilities|FlowControl|Sequence
            (:then_0
              (if (Variables|Default|GetRevengeOn)
                (CallFunction|Rotate (Variables|Default|GetRevengeEnemyPosition) 2.5e+02)
                (else
                  (CallFunction|Rotate (Variables|Default|GetEnemyPosition) 2.5e+02))))
            (:then_1
              ;[1 1 1] 攻撃モーション＆攻撃時間間隔
              (if (Variables|Default|GetAttackStart)
                (Utilities|FlowControl|DoOnce false :!label _label_2
                  (:Completed
                    (Default|Attack (Variables|Default|GetAnime))
                    (Collision|SetCollisionEnabled (Variables|Default|GetAttackCollision) "NoCollision")))))
            (:then_2
              (Utilities|FlowControl|Delay 2.0)
              (goto _label_2 Reset))
            (:then_3
              (goto _label))
            (:then_4
              ;[1 1 1] 攻撃中は歩きモーションをしない
              (Variables|/Game/Main/Blueprints/Yusya/Yusya04Anime.Yusya04Anime_C|SetIsWalk (Variables|Default|GetAnime) false))))))))

(event EventAttackCollisionReset
  ;[1 1 1] 攻撃中にキャンセルした時に当たり判定が残らないようにする
  (if (Variables|/Game/Main/Blueprints/Yusya/Yusya04Anime.Yusya04Anime_C|GetAttackOn (Variables|Default|GetAnime))
    (CallFunction|SetCollision true (Variables|Default|GetCapsule_0))
    (else
      (CallFunction|SetCollision false (Variables|Default|GetCapsule_0)))))

(fn ConstructionScript
  (|CallParentFunction))