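; Player castle that takes damage from attacking heroes (Yusya) and flags game over in GlobalInstance when its HP runs out.
; BlockBox applies tagged melee and bullet hits, briefly ignoring repeat melee from the last hero via a delayed ID reset on Tick.
; HaniBox toggles heroes' CastleIn flag, and TargetBox supplies random target points.
; Tick pushes the HP ratio to OrderUI; the widget bar's update and camera-facing calls are disconnected.
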(event OnComponentBeginOverlap(BlockBox)
  (params (OverlappedComponent :type Primitive%20Component%20Object%20Reference) (OtherActor :type Actor%20Object%20Reference) (OtherComp :type Primitive%20Component%20Object%20Reference) (OtherBodyIndex :type Integer) (bFromSweep :type Boolean) (SweepResult :type Hit%20Result%20Structure%20%28by%20ref%29))
  ;[1 1 1] 勇者の攻撃との当たり判定
  (Utilities|FlowControl|Sequence
    (:then_0
      (if (Components|ComponentHasTag OtherComp (Variables|/Game/Main/GlobalInstance.GlobalInstance_C|GetCollisionDamageTag (.AsGlobal%20Instance (Utilities|Casting|CastToGlobalInstance (Game|GetGameInstance)))))
        (bind _asyusya_oyaclass (Utilities|Casting|CastToYusyaOyaclass OtherActor))
        (if (!= (Variables|/Game/Main/Blueprints/Yusya/YusyaOyaclass.YusyaOyaclass_C|GetYusyaMyNumber _asyusya_oyaclass) (Variables|Default|GetStackYusyaNumber))
          (Variables|Default|SetStackYusyaNumber (Variables|/Game/Main/Blueprints/Yusya/YusyaOyaclass.YusyaOyaclass_C|GetYusyaMyNumber _asyusya_oyaclass))
          (bind _output_get (Variables|Default|SetHP (- (Variables|Default|GetHP) (Variables|/Game/Main/Blueprints/Yusya/YusyaOyaclass.YusyaOyaclass_C|GetStr _asyusya_oyaclass))))
          (if (<= _output_get 0.0)
            (Variables|Default|SetIsDeath true)
            (bind _asglobal_instance (Utilities|Casting|CastToGlobalInstance (Game|GetGameInstance)))
            (Variables|/Game/Main/GlobalInstance.GlobalInstance_C|SetGameOver _asglobal_instance true)))))
    (:then_1
      (if (Components|ComponentHasTag OtherComp (Variables|/Game/Main/GlobalInstance.GlobalInstance_C|GetCollisionBulletTag (.AsGlobal%20Instance (Utilities|Casting|CastToGlobalInstance (Game|GetGameInstance)))))
        (bind _asbullet_bp (Utilities|Casting|CastToBulletBP OtherActor))
        (bind _output_get_2 (Variables|Default|SetHP (- (Variables|Default|GetHP) (Variables|/Game/Main/Blueprints/Yusya/BulletBP.BulletBP_C|GetStr _asbullet_bp))))
        (Default|EndEmitter _asbullet_bp)
        (if (<= _output_get_2 0.0)
          (Variables|Default|SetIsDeath true)
          (bind _asglobal_instance_2 (Utilities|Casting|CastToGlobalInstance (Game|GetGameInstance)))
          (Variables|/Game/Main/GlobalInstance.GlobalInstance_C|SetGameOver _asglobal_instance_2 true))))))

(event OnComponentBeginOverlap(HaniBox)
  (params (OverlappedComponent :type Primitive%20Component%20Object%20Reference) (OtherActor :type Actor%20Object%20Reference) (OtherComp :type Primitive%20Component%20Object%20Reference) (OtherBodyIndex :type Integer) (bFromSweep :type Boolean) (SweepResult :type Hit%20Result%20Structure%20%28by%20ref%29))
  ;[1 1 1] 城の範囲内に勇者がはいったらtrue
  (if (Components|ComponentHasTag OtherComp (Variables|/Game/Main/GlobalInstance.GlobalInstance_C|GetCollisionYusyaTag (.AsGlobal%20Instance (Utilities|Casting|CastToGlobalInstance (Game|GetGameInstance)))))
    (bind _asyusya_oyaclass (Utilities|Casting|CastToYusyaOyaclass OtherActor))
    (Variables|/Game/Main/Blueprints/Yusya/YusyaOyaclass.YusyaOyaclass_C|SetCastleIn _asyusya_oyaclass true)))

(event OnComponentEndOverlap(HaniBox)
  (params (OverlappedComponent :type Primitive%20Component%20Object%20Reference) (OtherActor :type Actor%20Object%20Reference) (OtherComp :type Primitive%20Component%20Object%20Reference) (OtherBodyIndex :type Integer))
  ;[1 1 1] 城の範囲内に勇者がはいったらtrue
  (if (Components|ComponentHasTag OtherComp (Variables|/Game/Main/GlobalInstance.GlobalInstance_C|GetCollisionYusyaTag (.AsGlobal%20Instance (Utilities|Casting|CastToGlobalInstance (Game|GetGameInstance)))))
    (bind _asyusya_oyaclass (Utilities|Casting|CastToYusyaOyaclass OtherActor))
    (Variables|/Game/Main/Blueprints/Yusya/YusyaOyaclass.YusyaOyaclass_C|SetCastleIn _asyusya_oyaclass false)))

(event EventBeginPlay
  ;[1 1 1] コンポーネントタグに名前をセット
  (bind _asglobal_instance (Utilities|Casting|CastToGlobalInstance (Game|GetGameInstance)))
  (Utilities|Array|SetArrayElem (Variables|/Script/Engine.ActorComponent|GetComponentTags (Variables|Default|GetBlockBox)) 0 (Variables|/Game/Main/GlobalInstance.GlobalInstance_C|GetCollisionHaniAttackTag _asglobal_instance) true)
  (Variables|Default|SetHP (Variables|Default|GetMAXHP))
  (bind _ashp_ui (Utilities|Casting|CastToHP_UI (UserInterface|GetUserWidgetObject (Variables|Default|GetWidget))))
  (bind _output_get (Variables|Default|SetHPBAR_UI _ashp_ui))
  (Variables|/Game/Main/UI/HP_UI.HP_UI_C|SetHP _output_get 1.0))

(event Collision|EventActorBeginOverlap
  (params (OtherActor :type Actor%20Object%20Reference)))

(event EventTick
  (params (DeltaSeconds :type Float%20%28single-precision%29))
  ;[1 1 1] 2秒間は同じ勇者からダメージを受けない
  (Utilities|FlowControl|Sequence
    (:then_1
      ;[1 1 1] HPの割合を求めUIに送る
      (|HPWARIAI))
    (:then_2
      (if (> (Variables|Default|GetStackYusyaNumber) 0)
        (Utilities|FlowControl|Delay 2.0)
        (Variables|Default|SetStackYusyaNumber 0)))))

(fn ConstructionScript)

(fn GetCastleTargetPoint
  (bind _targetbox (Variables|Default|GetTargetBox))
  (bind (_origin _boxextent) (Collision|GetComponentBounds _targetbox))
  (return (Math|Random|RandomPointinBoundingBox _origin _boxextent)))