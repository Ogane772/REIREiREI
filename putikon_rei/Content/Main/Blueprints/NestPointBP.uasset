(event EventBeginPlay
  (bind _outactors (Actor|GetAllActorsOfClass "/Game/Main/Blueprints/StandbyInputActor.StandbyInputActor_C"))
  (for _array_element _outactors
    (Default|SetNestPointCount _array_element)
    (Rendering|SetVisibility (Variables|Default|Getyajirusi) false false)))

(event Collision|EventActorBeginOverlap
  (params (OtherActor :type Actor%20Object%20Reference)))

(event EventTick
  (params (DeltaSeconds :type Float%20%28single-precision%29))
  (Development|PrintString (Utilities|String|ToString(Integer) (Variables|Default|GetNestType)) true true "(R=0.000000,G=0.660000,B=1.000000,A=1.000000)" 0.0)
  (bind _新規track_0 (Timeline|タイムライン_0 Play)
    (:Update
      (Transformation|AddLocalOffset (Variables|Default|Getyajirusi) (Math|Vector|MakeVector 0.0 0.0 _新規track_0) false false))))

(fn ConstructionScript)

(fn SetYajirusiVisi
  (params (Visi :type Boolean))
  (Rendering|SetVisibility (Variables|Default|Getyajirusi) Visi false))

(fn SetParticleVisi
  (params (Visi :type Boolean))
  (Rendering|SetVisibility (Variables|Default|GetNiagara) Visi false))

(fn SetNestCreate
  (params (NestType :type Integer))
  (Variables|Default|SetNestType NestType)
  (CallFunction|SetParticleVisi false)
  (if (Variables|Default|GetIsNestON) ; すでに巣ができているときは前の巣を消す
    ;[1 1 1] もし巣を作っていたら作った巣を消す
    (bind _outactors (Actor|GetAllActorsOfClass "/Game/Main/Blueprints/Enemy/NestOyaclass.NestOyaclass_C"))
    (for _array_element _outactors
      (if (== (Variables|/Game/Main/Blueprints/Enemy/NestOyaclass.NestOyaclass_C|GetNestType _array_element) (Variables|Default|GetOldNestType))
        (Default|SetDestroy _array_element true)
        (bind _output_get (LocalVariables|SetTimeNestType (Variables|/Game/Main/Blueprints/Enemy/NestOyaclass.NestOyaclass_C|GetNestType _array_element)))
        (bind _output_get_2 (LocalVariables|SetTimeNestNumber (Variables|/Game/Main/Blueprints/Enemy/NestOyaclass.NestOyaclass_C|GetNestNumber _array_element)))))
    (CallFunction|NestCreate NestType true _output_get_2)
    (return true _output_get)
    (else
      (Variables|Default|SetIsNestON true)
      (CallFunction|NestCreate NestType false)
      (return false 0))))

(fn GetNestON
  (return (Variables|Default|GetIsNestON)))

(fn SetNestDelete
  (params (NesyNumber :type Integer) (Chenge :type Boolean))
  ;[1 1 1] 巣の番号と一致する巣を削除
  (bind _outactors (Actor|GetAllActorsOfClass "/Game/Main/Blueprints/Enemy/NestOyaclass.NestOyaclass_C"))
  (for _array_element _outactors
    (if (== (Variables|/Game/Main/Blueprints/Enemy/NestOyaclass.NestOyaclass_C|GetNestType _array_element) NesyNumber)
      (Default|SetDestroy _array_element Chenge))))

(fn SetNestON
  (params (isNestON :type Boolean))
  (Variables|Default|SetIsNestON isNestON)
  (if (not isNestON)
    (CallFunction|SetParticleVisi true)))

(fn NestCreate
  (params (Selection :type Integer) (Chenge :type Boolean) (ChengeNestNumber :type Integer))
  (bind _yajirusi (Variables|Default|Getyajirusi))
  (bind _defaultsceneroot (Variables|Default|GetDefaultSceneRoot))
  (bind _returnvalue (Transformation|GetWorldLocation _defaultsceneroot))
  (bind _returnvalue_2 (Transformation|GetWorldLocation _yajirusi))
  (bind _returnvalue_3 (Math|Conversions|ToTransform(Vector) _returnvalue))
  (if Chenge
    (LocalVariables|SetTimeNestNumber ChengeNestNumber)
    (else
      (LocalVariables|SetTimeNestNumber -1)))
  (switch int Selection
    (:1
      ;[1 1 1] 入れ替えたらネストカウントを増やさないのでtrueを返す
      (Game|SpawnActorfromClass "/Game/Main/Blueprints/Enemy/SrimeNest.SrimeNest_C" (Math|Conversions|ToTransform(Vector) _returnvalue) "Undefined" 0 (LocalVariables|GetTimeNestNumber) 0))
    (:2
      (Game|SpawnActorfromClass "/Game/Main/Blueprints/Enemy/TokageNest.TokageNest_C" _returnvalue_3 "Undefined" 0 (LocalVariables|GetTimeNestNumber) 0))
    (:3
      (Game|SpawnActorfromClass "/Game/Main/Blueprints/Enemy/RoboNest.RoboNest_C" _returnvalue_3 "Undefined" 0 (LocalVariables|GetTimeNestNumber) 0))
    (:4
      (Game|SpawnActorfromClass "/Game/Main/Blueprints/Enemy/GolemNest.GolemNest_C" _returnvalue_3 "Undefined" 0 (LocalVariables|GetTimeNestNumber) 0))
    (:5
      (Game|SpawnActorfromClass "/Game/Main/Blueprints/Enemy/GensanNest.GensanNest_C" _returnvalue_3 "Undefined" 0 (LocalVariables|GetTimeNestNumber) 0))
    (:6
      (Game|SpawnActorfromClass "/Game/Main/Blueprints/Enemy/BlackKnightNest.BlackKnightNest_C" _returnvalue_3 "Undefined" 0 (LocalVariables|GetTimeNestNumber) 0))
    (:7
      (Game|SpawnActorfromClass "/Game/Main/Blueprints/Enemy/DeathRoboNest.DeathRoboNest_C" _returnvalue_3 "Undefined" 0 (LocalVariables|GetTimeNestNumber) 0))
    (:8
      (Game|SpawnActorfromClass "/Game/Main/Blueprints/Enemy/TokageKnightNest.TokageKnightNest_C" _returnvalue_3 "Undefined" 0 (LocalVariables|GetTimeNestNumber) 0))
    (:9
      (Game|SpawnActorfromClass "/Game/Main/Blueprints/Enemy/MadousiNest.MadousiNest_C" _returnvalue_3 "Undefined" 0 (LocalVariables|GetTimeNestNumber) 0)))
  (Variables|Default|SetOldNestType (Variables|Default|GetNestType))
  (Niagara|SpawnSystematLocation "/Game/Main/particle/niagara/Monster/Monstar_Return/Return_1.Return_1" (Math|Vector|MakeVector (.x _returnvalue_2) (.y _returnvalue_2) (- (.z _returnvalue_2) 5.5e+02))))

(fn SetDestroy
  (Variables|Default|SetbAutoDestroyWhenFinished true)
  (Actor|SetLifeSpan 0.2))