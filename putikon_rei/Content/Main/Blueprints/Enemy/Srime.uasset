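; Slime enemy Blueprint that sets its stats and adds melee attack and death handling on top of a parent enemy class.
; Tick drives the SrimeAnime AnimInstance: in attack mode it turns toward the target and attacks on a DoOnce/Delay cooldown, otherwise it toggles walking.
; The animation's AttackON flag gates the Box1 hitbox, which damages YusyaOyaclass actors once per swing.
; Death disables collision, then finishes once the animation reports it.
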(event OnComponentBeginOverlap(Box1)
  (params (OverlappedComponent :type Primitive%20Component%20Object%20Reference) (OtherActor :type Actor%20Object%20Reference) (OtherComp :type Primitive%20Component%20Object%20Reference) (OtherBodyIndex :type Integer) (bFromSweep :type Boolean) (SweepResult :type Hit%20Result%20Structure%20%28by%20ref%29))
  ;[1 1 1] 攻撃中ならダメージを与える
  (if (Variables|/Game/Main/Blueprints/Enemy/SrimeAnime.SrimeAnime_C|GetAttackON (Variables|Default|GetAnime))
    (if (Utilities|ClassIsChildOf (Utilities|GetClass OtherActor) "/Game/Main/Blueprints/Yusya/YusyaOyaclass.YusyaOyaclass_C")
      (Game|Damage|ApplyDamage OtherActor (Variables|Default|GetStr) 0 0)
      (Variables|/Game/Main/Blueprints/Enemy/SrimeAnime.SrimeAnime_C|SetAttackON (Variables|Default|GetAnime) false))))

(event EventBeginPlay
  ;[1 1 1] BeginPlay
  (|CallParentFunction)
  (Variables|Default|SetEnemyType "NewEnumerator0")
  (bind _assrime_anime (Utilities|Casting|CastToSrimeAnime (Components|SkeletalMesh|GetAnimInstance (Variables|Default|GetSkeletalMesh))))
  (Variables|Default|SetAnime _assrime_anime)
  (Variables|Default|SetStr 1.0)
  (CallFunction|SetCollision false (Variables|Default|GetBox1))
  (bind _output_get (Variables|Default|SetMAXHP 1e+01))
  (Variables|Default|SetHP _output_get))

(event Collision|EventActorBeginOverlap
  (params (OtherActor :type Actor%20Object%20Reference))
  (|CallParentFunction OtherActor))

(event EventTick
  (params (DeltaSeconds :type Float%20%28single-precision%29))
  (bind _box1 (Variables|Default|GetBox1))
  (Development|PrintString (Utilities|String|ToString(Float) (Variables|Default|GetHP)) true true "(R=0.000000,G=0.660000,B=1.000000,A=1.000000)" 0.0)
  (if (Variables|Default|GetIsDeath)
    ;[1 1 1] 死亡時の処理
    (Utilities|FlowControl|Sequence
      (:then_0
        (Utilities|FlowControl|DoOnce false
          (:Completed
            (Default|Death (Variables|Default|GetAnime))
            (CallFunction|SetCollision false (Variables|Default|GetBox1))
            (CallFunction|SetCollision false (Variables|Default|GetBox)))))
      (:then_1
        (if (Variables|/Game/Main/Blueprints/Enemy/SrimeAnime.SrimeAnime_C|GetIsDeath (Variables|Default|GetAnime))
          (CallFunction|EnemyDeath)
          (Variables|Default|SetbAutoDestroyWhenFinished true))))
    (else
      (Utilities|FlowControl|Sequence
        (:then_0
          (|CallParentFunction DeltaSeconds)
          (if (Variables|Default|GetAttackMode)
            (Variables|/Game/Main/Blueprints/Enemy/SrimeAnime.SrimeAnime_C|SetIsWalk (Variables|Default|GetAnime) false)
            (Utilities|FlowControl|Sequence
              (:then_0
                (CallFunction|Rotate (Variables|Default|GetTargetPosition) 4e+02))
              (:then_1
                ;[1 1 1] 攻撃モーション＆攻撃時間間隔
                (Utilities|FlowControl|DoOnce false :!label _label
                  (:Completed
                    (Default|Attack (Variables|Default|GetAnime)))))
              (:then_2
                (Utilities|FlowControl|Delay 2.4)
                (goto _label Reset))
              (:then_3
                ;[1 1 1] 攻撃モーションの当たり判定更新
                (if (Variables|/Game/Main/Blueprints/Enemy/SrimeAnime.SrimeAnime_C|GetAttackON (Variables|Default|GetAnime))
                  (CallFunction|SetCollision true _box1)
                  (else
                    (CallFunction|SetCollision false _box1)))))
            (elif (Variables|Default|GetMoveStop)
              (Variables|/Game/Main/Blueprints/Enemy/SrimeAnime.SrimeAnime_C|SetIsWalk (Variables|Default|GetAnime) false)
              (else
                (Variables|/Game/Main/Blueprints/Enemy/SrimeAnime.SrimeAnime_C|SetIsWalk (Variables|Default|GetAnime) true)))))
        (:then_1
          (Variables|Default|SetNoMove (Variables|/Game/Main/Blueprints/Enemy/SrimeAnime.SrimeAnime_C|GetNoMove (Variables|Default|GetAnime))))))))

(fn ConstructionScript
  (|CallParentFunction))