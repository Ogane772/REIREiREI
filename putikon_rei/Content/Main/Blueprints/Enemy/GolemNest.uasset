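; GolemNest is an enemy nest Blueprint configured to produce Golem enemies.
; On BeginPlay it sets the enemy class and type, then reads row "4" of the EnemyData table for name, nest limit, timing, starting count, HP and type number.
; Parent BeginPlay runs only after the row is found, so the parent class handles the nest behavior using these values.
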(event EventBeginPlay
  (Variables|Default|SetEnemyClass "/Game/Main/Blueprints/Enemy/Golem/Golem.Golem_C")
  (Variables|Default|SetEnemyType "NewEnumerator4")
  (bind _returnvalue (Utilities|GetDataTableRow "/Game/Main/CSV/EnemyData.EnemyData" "4")
    (:then
      (Variables|Default|SetEnemyName (.Name (Utilities|Struct|BreakEnemyDataTable _returnvalue)))
      (Variables|Default|SetMAX_NESTNUM (.MAXNUM (Utilities|Struct|BreakEnemyDataTable _returnvalue)))
      (Variables|Default|SetNestTime (.NestTime (Utilities|Struct|BreakEnemyDataTable _returnvalue)))
      (Variables|Default|SetEnemyNestNum (.FirstNum (Utilities|Struct|BreakEnemyDataTable _returnvalue)))
      (bind _output_get (Variables|Default|SetMAXHP (.NestHP (Utilities|Struct|BreakEnemyDataTable _returnvalue))))
      (Variables|Default|SetHP _output_get)
      (Variables|Default|SetNestType (.Number (Utilities|Struct|BreakEnemyDataTable _returnvalue)))
      (|CallParentFunction))))

(event Collision|EventActorBeginOverlap
  (params (OtherActor :type Actor%20Object%20Reference))
  (|CallParentFunction OtherActor) ; This node is disabled and will not be called.\nDrag off pins to build functionality.
)

(event EventTick
  (params (DeltaSeconds :type Float%20%28single-precision%29))
  (|CallParentFunction DeltaSeconds) ; This node is disabled and will not be called.\nDrag off pins to build functionality.
)

(fn ConstructionScript
  (|CallParentFunction))