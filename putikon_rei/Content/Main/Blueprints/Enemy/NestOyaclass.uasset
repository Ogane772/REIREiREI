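; Base monster nest that registers with the shared order UI, breeds population, spawns slimes or lizards, and relays orders to enemies of its type.
; Looping timers grow the population under the breed order while none are fielded, otherwise spawn up to that count inside SpawnBox; zero population forces breeding.
; BlockBox takes hero damage, debounced by hero number, while SpawnBox flags heroes inside.
; Tick updates the camera-facing HP display.
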(event OnComponentBeginOverlap(BlockBox)
  (params (OverlappedComponent :type Primitive%20Component%20Object%20Reference) (OtherActor :type Actor%20Object%20Reference) (OtherComp :type Primitive%20Component%20Object%20Reference) (OtherBodyIndex :type Integer) (bFromSweep :type Boolean) (SweepResult :type Hit%20Result%20Structure%20%28by%20ref%29))
  ;[1 1 1] 勇者の攻撃との当たり判定
  (if (Components|ComponentHasTag OtherComp (Variables|/Game/Main/GlobalInstance.GlobalInstance_C|GetCollisionDamageTag (.AsGlobal%20Instance (Utilities|Casting|CastToGlobalInstance (Game|GetGameInstance)))))
    (bind _asyusya_oyaclass (Utilities|Casting|CastToYusyaOyaclass OtherActor))
    (if (!= (Variables|/Game/Main/Blueprints/Yusya/YusyaOyaclass.YusyaOyaclass_C|GetYusyaMyNumber _asyusya_oyaclass) (Variables|Default|GetStackYusyaNumber))
      (Variables|Default|SetStackYusyaNumber (Variables|/Game/Main/Blueprints/Yusya/YusyaOyaclass.YusyaOyaclass_C|GetYusyaMyNumber _asyusya_oyaclass))
      (bind _output_get (Variables|Default|SetHP (- (Variables|Default|GetHP) (Variables|/Game/Main/Blueprints/Yusya/YusyaOyaclass.YusyaOyaclass_C|GetStr _asyusya_oyaclass))))
      (if (<= _output_get 0.0)
        (Variables|Default|SetIsDeath true)))))

(event OnComponentBeginOverlap(SpawnBox)
  (params (OverlappedComponent :type Primitive%20Component%20Object%20Reference) (OtherActor :type Actor%20Object%20Reference) (OtherComp :type Primitive%20Component%20Object%20Reference) (OtherBodyIndex :type Integer) (bFromSweep :type Boolean) (SweepResult :type Hit%20Result%20Structure%20%28by%20ref%29))
  ;[1 1 1] 巣の範囲内に勇者がはいったらtrue
  (if (Components|ComponentHasTag OtherComp (Variables|/Game/Main/GlobalInstance.GlobalInstance_C|GetCollisionYusyaTag (.AsGlobal%20Instance (Utilities|Casting|CastToGlobalInstance (Game|GetGameInstance)))))
    (bind _asyusya_oyaclass (Utilities|Casting|CastToYusyaOyaclass OtherActor))
    (Variables|/Game/Main/Blueprints/Yusya/YusyaOyaclass.YusyaOyaclass_C|SetNestIn _asyusya_oyaclass true)))

(event OnComponentEndOverlap(SpawnBox)
  (params (OverlappedComponent :type Primitive%20Component%20Object%20Reference) (OtherActor :type Actor%20Object%20Reference) (OtherComp :type Primitive%20Component%20Object%20Reference) (OtherBodyIndex :type Integer))
  ;[1 1 1] 巣の範囲内に勇者がはいったらtrue
  (if (Components|ComponentHasTag OtherComp (Variables|/Game/Main/GlobalInstance.GlobalInstance_C|GetCollisionYusyaTag (.AsGlobal%20Instance (Utilities|Casting|CastToGlobalInstance (Game|GetGameInstance)))))
    (bind _asyusya_oyaclass (Utilities|Casting|CastToYusyaOyaclass OtherActor))
    (Variables|/Game/Main/Blueprints/Yusya/YusyaOyaclass.YusyaOyaclass_C|SetNestIn _asyusya_oyaclass false)))

(event Custom|EnemySpawn
  (bind _spawnbox (Variables|Default|GetSpawnBox))
  (bind (_origin _boxextent) (Collision|GetComponentBounds _spawnbox))
  (bind _returnvalue (Math|Random|RandomPointinBoundingBox _origin _boxextent))
  (bind _returnvalue_2 (Math|Conversions|ToTransform(Vector) _returnvalue))
  ;[1 1 1] エネミースポーン処理
  (if (< (Variables|Default|GetEnemyFieldCount) (Variables|Default|GetMAX_NESTNUM))
    (if (< (Variables|Default|GetEnemyFieldCount) (Variables|Default|GetEnemyNestNum)) ; フィールドに出ている数が総数より下だったら生成
      (if (Utilities|Enum|NotEqual(Enum) (Variables|Default|GetOrderNumber) "NewEnumerator3") ; 命令が繁殖する以外ならスポーン
        (switch Utilities|FlowControl|Switch|SwitchonEnemyTypeEnum (Variables|Default|GetEnemyType)
          (:NewEnumerator0
            (Game|SpawnActorfromClass "/Game/Main/Blueprints/Enemy/srime/Srime.Srime_C" _returnvalue_2 "Undefined" 0 (Variables|Default|GetOrderNumber) 0))
          (:NewEnumerator2
            (Game|SpawnActorfromClass "/Game/Main/Blueprints/Enemy/Tokage/Tokage.Tokage_C" _returnvalue_2 "Undefined" 0 (Variables|Default|GetOrderNumber) 0)))
        (bind _result (Math|Integer|IncrementInt (Variables|Default|GetEnemyFieldCount))
          (:%20%20
            (Variables|Default|SetEnemyFieldCount _result)))))))

(event Custom|EnemyPurasu
  (bind _nestnumber (Variables|Default|GetNestNumber))
  ;[1 1 1] 命令が繁殖なら一定時間ごとにエネミーを増やす
  (if (Utilities|Enum|Equal(Enum) (Variables|Default|GetOrderNumber) "NewEnumerator3")
    (if (< (Variables|Default|GetEnemyNestNum) (Variables|Default|GetMAX_NESTNUM))
      (if (== (Variables|Default|GetEnemyFieldCount) 0)
        (bind _result (Math|Integer|IncrementInt (Variables|Default|GetEnemyNestNum))
          (:%20%20
            (bind _output_get (Variables|Default|SetEnemyNestNum _result))
            (Default|SeｔEnemyNum (Variables|/Game/Main/GlobalInstance.GlobalInstance_C|GetOrderUI (stale EventBeginPlay _asglobal_instance_2)) _output_get _nestnumber)
            (if (== (Variables|Default|GetEnemyNestNum) 1) ; 0から1になったら命令ロック解除
              (bind _asglobal_instance (Utilities|Casting|CastToGlobalInstance (Game|GetGameInstance)))
              (Default|SetOrderLock (Variables|/Game/Main/GlobalInstance.GlobalInstance_C|GetOrderUI _asglobal_instance) false _nestnumber))))))))

(event EventBeginPlay
  (bind _ashp_ui (Utilities|Casting|CastToHP_UI (UserInterface|GetUserWidgetObject (Variables|Default|GetHP_BAR))))
  (bind _output_get (Variables|Default|SetHPBAR_UI _ashp_ui))
  (Variables|/Game/Main/HP_UI.HP_UI_C|SetHP _output_get 1.0)
  ;[1 1 1] コンポーネントタグに名前をセット
  (bind _asglobal_instance (Utilities|Casting|CastToGlobalInstance (Game|GetGameInstance)))
  (Utilities|Array|SetArrayElem (Variables|/Script/Engine.ActorComponent|GetComponentTags (Variables|Default|GetSpawnBox)) 0 (Variables|/Game/Main/GlobalInstance.GlobalInstance_C|GetCollisionHaniTag _asglobal_instance) true)
  ;[1 1 1] コンポーネントタグに名前をセット
  (bind _asglobal_instance_2 (Utilities|Casting|CastToGlobalInstance (Game|GetGameInstance)))
  (Utilities|Array|SetArrayElem (Variables|/Script/Engine.ActorComponent|GetComponentTags (Variables|Default|GetBlockBox)) 0 (Variables|/Game/Main/GlobalInstance.GlobalInstance_C|GetCollisionNestTag _asglobal_instance_2) true)
  ;[1 1 1] コンポーネントタグに名前をセット
  (bind _asglobal_instance_3 (Utilities|Casting|CastToGlobalInstance (Game|GetGameInstance)))
  (Utilities|Array|SetArrayElem (Variables|/Script/Engine.ActorComponent|GetComponentTags (Variables|Default|GetBlockBox)) 1 (Variables|/Game/Main/GlobalInstance.GlobalInstance_C|GetCollisionHaniAttackTag _asglobal_instance_3) true)
  (Utilities|Time|SetTimerbyEvent (delegate Custom|EnemyPurasu) (Variables|Default|GetNestTime) true)
  (Utilities|Time|SetTimerbyEvent (delegate Custom|EnemySpawn) 2.0 true)
  (Utilities|IsValid (Variables|/Game/Main/GlobalInstance.GlobalInstance_C|GetOrderUI _asglobal_instance_2) ; UIが存在しなかったらUI作成
    (:Is%20Valid
      _)
    (:Is%20Not%20Valid
      (bind _returnvalue (UserInterface|CreateWidget "/Game/Main/MonsterUI.MonsterUI_C"))
      (bind _output_get_2 (Variables|/Game/Main/GlobalInstance.GlobalInstance_C|SetOrderUI _asglobal_instance_2 _returnvalue))
      (UserInterface|Viewport|AddtoViewport _output_get_2 0)))
  ;[1 1 1] 現在存在しているエネミーの総数を数える
  (bind _outactors (Actor|GetAllActorsOfClass (Variables|Default|GetEnemyClass)))
  (for _array_element _outactors
    (bind _result (Math|Integer|IncrementInt (Variables|Default|GetEnemyFieldCount))
      (:%20%20
        (Variables|Default|SetEnemyFieldCount _result))))
  (bind _output_get_3 (Variables|Default|SetEnemyNestNum (+ (Variables|Default|GetEnemyFieldCount) (Variables|Default|GetEnemyNestNum))))
  (bind _nestnumber (Default|SetEnemyData (Variables|/Game/Main/GlobalInstance.GlobalInstance_C|GetOrderUI _asglobal_instance_2) (Variables|Default|GetEnemyName) _output_get_3 (Variables|Default|GetMAX_NESTNUM) (Variables|Default|GetEnemyType))) ; UIにエネミーデータを登録
  (Math|Integer|DecrementInt _nestnumber
    (:%20%20
      (Variables|Default|SetNestNumber _nestnumber) ; UIから巣の識別番号を受け取る
    )))

(event Collision|EventActorBeginOverlap
  (params (OtherActor :type Actor%20Object%20Reference))
  ;[1 1 1] コンポーネントタグに名前をセット
)

(event EventTick
  (params (DeltaSeconds :type Float%20%28single-precision%29))
  (Development|PrintString (Utilities|String|ToString(Integer) (Variables|Default|GetNestNumber)) true true "(R=1.000000,G=0.983748,B=0.660982,A=1.000000)" 0.0)
  (Utilities|FlowControl|Sequence
    (:then_0
      ;[1 1 1] HPゲージが常にカメラを向くように設定
      (|CameraMove_2))
    (:then_1
      ;[1 1 1] HPの割合を求める
      (|HP＿WARIAI_2))
    (:then_2
      (if (> (Variables|Default|GetStackYusyaNumber) 0)
        (Utilities|FlowControl|Delay 2.0)
        (Variables|Default|SetStackYusyaNumber 0)))))

(fn ConstructionScript)

(fn SetOrderNumber
  (params (NewParam :type EnemyOrderEnum%20Enum :default "NewEnumerator0"))
  ;[1 1 1] 命令番号を更新し自分の召喚するモンスターに命令番号を渡す
  (bind _output_get (Variables|Default|SetOrderNumber NewParam))
  (bind _outactors (Actor|GetAllActorsOfClass "/Game/Main/Blueprints/Enemy/EnemyOyaclass.EnemyOyaclass_C"))
  (for _array_element _outactors
    (if (Utilities|Enum|Equal(Enum) (Variables|/Game/Main/Blueprints/Enemy/EnemyOyaclass.EnemyOyaclass_C|GetEnemyType _array_element) (Variables|Default|GetEnemyType))
      (Default|SetOrderNumber _array_element _output_get))))

(fn SetEnemyCountMinus
  (bind _result (Math|Integer|DecrementInt (Variables|Default|GetEnemyFieldCount))
    (:%20%20
      (bind _output_get (Variables|Default|SetEnemyFieldCount _result))
      (if (< _output_get 0)
        (Variables|Default|SetEnemyFieldCount 0)))))

(fn GetEnemyTargetPoint
  (bind _spawnbox (Variables|Default|GetSpawnBox))
  (bind (_origin _boxextent) (Collision|GetComponentBounds _spawnbox))
  (return (Math|Random|RandomPointinBoundingBox _origin _boxextent)))

(fn SetEnemyDelete
  (Utilities|FlowControl|Sequence
    (:then_0
      (bind _result (Math|Integer|DecrementInt (Variables|Default|GetEnemyFieldCount))
        (:%20%20
          (bind _output_get (Variables|Default|SetEnemyFieldCount _result))
          (if (< _output_get 0)
            (Variables|Default|SetEnemyFieldCount 0)))))
    (:then_1
      (bind _result_2 (Math|Integer|DecrementInt (Variables|Default|GetEnemyNestNum))
        (:%20%20
          (bind _output_get_2 (Variables|Default|SetEnemyNestNum _result_2))
          (if (< _output_get_2 0)
            (Variables|Default|SetEnemyNestNum 0))
          (bind _asglobal_instance (Utilities|Casting|CastToGlobalInstance (Game|GetGameInstance)))
          (Default|SeｔEnemyNum (Variables|/Game/Main/GlobalInstance.GlobalInstance_C|GetOrderUI _asglobal_instance) (Variables|Default|GetEnemyNestNum) (Variables|Default|GetNestNumber)))))
    (:then_2
      (if (== (Variables|Default|GetEnemyNestNum) 0) ; 数が0以下なら命令を繁栄するにする
        (Variables|Default|SetOrderNumber "NewEnumerator3")
        (bind _asglobal_instance_2 (Utilities|Casting|CastToGlobalInstance (Game|GetGameInstance)))
        (Default|SetOrderHanei (Variables|/Game/Main/GlobalInstance.GlobalInstance_C|GetOrderUI _asglobal_instance_2) (Variables|Default|GetNestNumber))))))