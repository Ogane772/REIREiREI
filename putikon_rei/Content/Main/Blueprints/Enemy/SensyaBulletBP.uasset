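; Enemy tank (Sensya) bullet that flies toward a target position and damages the hero (YusyaOyaclass).
; BeginPlay tags its collision as a bullet and faces the mesh at the target; Tick steps it at constant per-frame speed, ignoring delta time.
; Tagged hero overlaps apply damage and spawn an explosion, as does EndEmitter without damage.
; Hits, EndEmitter and X/Y arrival hide the mesh and set AutoDestroyWhenFinished; smooth-turn logic is unconnected.
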(event OnComponentBeginOverlap(AttackCollision)
  (params (OverlappedComponent :type Primitive%20Component%20Object%20Reference) (OtherActor :type Actor%20Object%20Reference) (OtherComp :type Primitive%20Component%20Object%20Reference) (OtherBodyIndex :type Integer) (bFromSweep :type Boolean) (SweepResult :type Hit%20Result%20Structure%20%28by%20ref%29))
  (bind _asglobal_instance (Utilities|Casting|CastToGlobalInstance (Game|GetGameInstance)))
  (if (Components|ComponentHasTag OtherComp (Variables|/Game/Main/GlobalInstance.GlobalInstance_C|GetCollisionYusyaTag _asglobal_instance))
    (bind _asyusya_oyaclass (Utilities|Casting|CastToYusyaOyaclass OtherActor))
    (Default|Damage _asyusya_oyaclass (Variables|Default|GetStr) true)
    (Niagara|SpawnSystematLocation "/Game/Main/particle/niagara/Monster/Monstar_attack/Tank_Attack/Explosion_2.Explosion_2" (Transformation|GetWorldLocation (Variables|Default|GetStaticMesh)))
    (Rendering|SetVisibility (Variables|Default|GetStaticMesh) false false)
    (Variables|Default|SetbAutoDestroyWhenFinished true)))

(event Custom|EndEmitter
  (Niagara|SpawnSystematLocation "/Game/Main/particle/niagara/Monster/Monstar_attack/Tank_Attack/Explosion_2.Explosion_2" (Transformation|GetWorldLocation (Variables|Default|GetStaticMesh)))
  (Rendering|SetVisibility (Variables|Default|GetStaticMesh) false false)
  (Variables|Default|SetbAutoDestroyWhenFinished true))

(event EventBeginPlay
  (bind _output_get (Variables|Default|SetMoveSpeed 4e+01))
  (Variables|Default|SetHitLength _output_get)
  (bind _asglobal_instance (Utilities|Casting|CastToGlobalInstance (Game|GetGameInstance)))
  (Utilities|Array|SetArrayElem (Variables|/Script/Engine.ActorComponent|GetComponentTags (Variables|Default|GetAttackCollision)) 0 (Variables|/Game/Main/GlobalInstance.GlobalInstance_C|GetCollisionBulletTag _asglobal_instance) true)
  (Transformation|SetWorldRotation (Variables|Default|GetStaticMesh) (Math|Rotator|FindLookatRotation (Transformation|GetWorldLocation (Variables|Default|GetStaticMesh)) (Variables|Default|GetTargetPositiom)) false false))

(event Collision|EventActorBeginOverlap
  (params (OtherActor :type Actor%20Object%20Reference)))

(event EventTick
  (params (DeltaSeconds :type Float%20%28single-precision%29))
  (bind _targetpositiom (Variables|Default|GetTargetPositiom))
  (bind _staticmesh (Variables|Default|GetStaticMesh))
  (if (Rendering|IsVisible (Variables|Default|GetStaticMesh))
    (Utilities|FlowControl|Sequence
      (:then_0
        (bind _output_get (Variables|Default|SetStackPosition (- (Variables|Default|GetTargetPositiom) (Transformation|GetWorldLocation (Variables|Default|GetStaticMesh)))))
        (Transformation|SetWorldLocation _staticmesh (+ (* (Math|Vector|Normalize _output_get) (Variables|Default|GetMoveSpeed)) (Transformation|GetWorldLocation _staticmesh)) false false))
      (:then_1
        ;[1 1 1] ターゲットの位置に着いているか判定
        (if (>= (+ (.x _targetpositiom) (Variables|Default|GetHitLength)) (.x (Transformation|GetWorldLocation (Variables|Default|GetStaticMesh))))
          (if (<= (- (.x _targetpositiom) (Variables|Default|GetHitLength)) (.x (Transformation|GetWorldLocation (Variables|Default|GetStaticMesh))))
            (if (>= (+ (.y _targetpositiom) (Variables|Default|GetHitLength)) (.y (Transformation|GetWorldLocation (Variables|Default|GetStaticMesh))))
              (if (<= (- (.y _targetpositiom) (Variables|Default|GetHitLength)) (.y (Transformation|GetWorldLocation (Variables|Default|GetStaticMesh))))
                (Rendering|SetVisibility (Variables|Default|GetStaticMesh) false false)
                (Variables|Default|SetbAutoDestroyWhenFinished true)))))))))

(fn ConstructionScript)