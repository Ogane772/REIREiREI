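; EnemyOyaclass is the parent enemy actor that acts on a numbered order: battle, nest guard, castle guard or breeding.
; SetOrderNumber picks fixed targets, while Battle chases the nearest hero (Yusya), falling back to the nest.
; Tick moves straight with axis-angle turning, then faces the Castle on arrival, and updates a camera-facing HP text.
; Box overlaps trigger attack mode or nest return; damage briefly ignores repeat hits from one hero.
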(event OnComponentBeginOverlap(Box)
  (params (OverlappedComponent :type Primitive%20Component%20Object%20Reference) (OtherActor :type Actor%20Object%20Reference) (OtherComp :type Primitive%20Component%20Object%20Reference) (OtherBodyIndex :type Integer) (bFromSweep :type Boolean) (SweepResult :type Hit%20Result%20Structure%20%28by%20ref%29))
  ;[1 1 1] 当たり判定
  (Utilities|FlowControl|Sequence
    (:then_1
      ;;[1 1 1] 命令番号が巣に戻るの時エネミーカウントをマイナスしデストロイする
      (bind _asglobal_instance (Utilities|Casting|CastToGlobalInstance (Game|GetGameInstance)))
      (if (Components|ComponentHasTag OtherComp (Variables|/Game/Main/GlobalInstance.GlobalInstance_C|GetCollisionNestTag _asglobal_instance))
        (if (Utilities|Enum|Equal(Enum) (Variables|Default|GetOrderNumber) "NewEnumerator3")
          (bind _outactors (Actor|GetAllActorsOfClass "/Game/Main/Blueprints/Enemy/NestOyaclass.NestOyaclass_C"))
          (for _array_element _outactors
            (Default|SetEnemyCountMinus _array_element))
          (Variables|Default|SetbAutoDestroyWhenFinished true))))
    (:then_2
      ;;[1 1 1] 命令がたたかうの時勇者に当たったらバトルモード(後で巣を守るや城を守るときはその周辺に来たやつを攻撃するようにする)
      (bind _asglobal_instance_2 (Utilities|Casting|CastToGlobalInstance (Game|GetGameInstance)))
      (if (Components|ComponentHasTag OtherComp (Variables|/Game/Main/GlobalInstance.GlobalInstance_C|GetCollisionYusyaTag _asglobal_instance_2))
        (if (Utilities|Enum|Equal(Enum) (Variables|Default|GetOrderNumber) "NewEnumerator0")
          (Variables|Default|SetAttackMode true)
          (Variables|Default|SetMoveStop true)
          (bind _asyusya_oyaclass (Utilities|Casting|CastToYusyaOyaclass OtherActor))
          (Variables|Default|SetBattleYusyaPosition (Transformation|GetWorldLocation (Variables|/Game/Main/Blueprints/Yusya/YusyaOyaclass.YusyaOyaclass_C|GetBox1 _asyusya_oyaclass))))))))

(event OnComponentEndOverlap(Box)
  (params (OverlappedComponent :type Primitive%20Component%20Object%20Reference) (OtherActor :type Actor%20Object%20Reference) (OtherComp :type Primitive%20Component%20Object%20Reference) (OtherBodyIndex :type Integer))
  ;[1 1 1] 当たり判定
  (bind _asglobal_instance (Utilities|Casting|CastToGlobalInstance (Game|GetGameInstance)))
  (if (Components|ComponentHasTag OtherComp (Variables|/Game/Main/GlobalInstance.GlobalInstance_C|GetCollisionYusyaTag _asglobal_instance))
    (Variables|Default|SetAttackMode false)
    (Variables|Default|SetMoveStop false)))

(event Custom|DamageEvent
  (params (damage :type Float%20%28single-precision%29) (YusyaNumber :type Integer))
  ;[1 1 1] ダメージ処理（勇者ナンバーが同じならダメージを受けない
  (if (!= YusyaNumber (Variables|Default|GetDamageYusyaNumber))
    (Variables|Default|SetHP (- (Variables|Default|GetHP) damage))
    (Variables|Default|SetDamageYusyaNumber YusyaNumber)
    (if (<= (Variables|Default|GetHP) 0.0) ; HPが0以下で死亡フラグを立てる
      (Variables|Default|SetIsDeath true))))

(event Custom|EnemyDeath
  ;[1 1 1] エネミーが死亡時は親の巣に死亡したと通知する
  (switch Utilities|FlowControl|Switch|SwitchonEnemyTypeEnum (Variables|Default|GetEnemyType)
    (:NewEnumerator0
      (bind _outactors (Actor|GetAllActorsOfClass "/Game/Main/Blueprints/Enemy/SrimeNest.SrimeNest_C"))
      (for _array_element _outactors
        (Default|SetEnemyDelete _array_element)))))

(event EventBeginPlay
  (CallFunction|SetOrderNumber (Variables|Default|GetOrderNumber))
  ;[1 1 1] 待機時敵の城の方を向くため位置を保存
  (bind _outactors (Actor|GetAllActorsOfClass "/Game/Main/Blueprints/castle.castle_C"))
  (for _array_element _outactors
    (Variables|Default|SetYusyaCastlePosition (Transformation|GetWorldLocation (Variables|/Game/Main/Blueprints/castle.castle_C|GetStaticMesh _array_element)))
    ;[1 1 1] コンポーネントタグに名前をセット
    (bind _asglobal_instance (Utilities|Casting|CastToGlobalInstance (Game|GetGameInstance)))
    (Utilities|Array|SetArrayElem (Variables|/Script/Engine.ActorComponent|GetComponentTags (Variables|コンポーネント|GetBox)) 0 (Variables|/Game/Main/GlobalInstance.GlobalInstance_C|GetCollisionEnemyTag _asglobal_instance) true)
    ;[1 1 1] 命令が実行できないときは巣に戻るため位置を取得
    (bind _outactors_2 (Actor|GetAllActorsOfClass "/Game/Main/Blueprints/Enemy/NestOyaclass.NestOyaclass_C"))
    (for _array_element_2 _outactors_2
      (bind _targetpoint (Default|GetEnemyTargetPoint _array_element_2))
      (Variables|Default|SetStartNestPosition _targetpoint))))

(event Collision|EventActorBeginOverlap
  (params (OtherActor :type Actor%20Object%20Reference)))

(event EventTick
  (params (DeltaSeconds :type Float%20%28single-precision%29))
  (Utilities|IsValid (Variables|Default|GetSkeletalMesh)
    (:Is%20Valid
      (Utilities|FlowControl|Sequence
        (:then_0
          ;[1 1 1] HPゲージが常にカメラを向くように設定
          (|CameraMove_2_2_2))
        (:then_1
          ;[1 1 1] HPの割合を求める
          (|HP＿WARIAI_2_2_2))
        (:then_2
          (if (Utilities|Enum|Equal(Enum) (Variables|Default|GetCollisionType) "NoCollision")
            (bind _output_get (Variables|Default|SetCollisionType "QueryAndPhysics"))
            (Collision|SetCollisionEnabled (Variables|コンポーネント|GetBox) _output_get))
          (Utilities|FlowControl|Sequence
            (:then_0
              (if (not (Variables|Default|GetAttackMode))
                (if (not (Variables|Default|GetMoveStop))
                  (if (not (Variables|Default|GetNoMove))
                    (switch Utilities|FlowControl|Switch|SwitchonEnemyOrderEnum (Variables|Default|GetOrderNumber) ; 命令毎の行動
                      (:NewEnumerator0
                        (Utilities|FlowControl|Sequence
                          (:then_0
                            ;[1 1 1] 一番近い勇者の場所に行く
                            (bind _yusyaposition (CallFunction|GetYusyaPosition))
                            (Variables|Default|SetTargetPosition _yusyaposition))
                          (:then_1
                            ;[1 1 1] 対象まで直線で移動
                            (CallFunction|TargetMove (Variables|Default|GetMoveSpeed)))))
                      (:NewEnumerator1
                        (Utilities|FlowControl|Sequence
                          (:then_0
                            ;[1 1 1] 対象まで直線で移動
                            (CallFunction|TargetMove (Variables|Default|GetMoveSpeed)))))
                      (:NewEnumerator2
                        (Utilities|FlowControl|Sequence
                          (:then_1
                            ;[1 1 1] 対象まで直線で移動
                            (CallFunction|TargetMove (Variables|Default|GetMoveSpeed)))))
                      (:NewEnumerator3
                        (Utilities|FlowControl|Sequence
                          (:then_0
                            ;[1 1 1] 対象まで直線で移動
                            (CallFunction|TargetMove (Variables|Default|GetMoveSpeed)))))))
                  (else
                    ;[1 1 1] ポイントに着いたら敵の城の方を向く
                    (CallFunction|YusyaCastleRotate (Variables|Default|GetSkeletalMesh))))))
            (:then_1
              ;[1 1 1] ターゲットの位置に着いているか判定
              (CallFunction|TargetPointCheck (Variables|Default|GetHitLength)))
            (:then_3
              ;[1 1 1] 2秒間は同じ勇者からダメージを受けない
              (if (> (Variables|Default|GetDamageYusyaNumber) 0)
                (Utilities|FlowControl|Delay 2.0)
                (Variables|Default|SetDamageYusyaNumber 0)))))))))

(fn ConstructionScript)

(fn TargetMove
  (params (movespeed :type Float%20%28single-precision%29))
  (bind _skeletalmesh (Variables|Default|GetSkeletalMesh))
  (bind _skeletalmesh_2 (Variables|Default|GetSkeletalMesh))
  (bind _returnvalue (Transformation|GetWorldRotation _skeletalmesh_2))
  (bind _returnvalue_2 (Transformation|GetWorldLocation _skeletalmesh))
  (bind _output_get (Variables|Default|SetStackPosition (- (Variables|Default|GetTargetPosition) (Transformation|GetWorldLocation (Variables|Default|GetSkeletalMesh)))))
  (Transformation|SetWorldLocation (Variables|Default|GetSkeletalMesh) (+ (* (Math|Vector|Normalize _output_get) movespeed) _returnvalue_2) true false)
  ;[1 1 1] 徐々にターゲットの方に回転させる
  (Transformation|SetWorldRotation (Variables|Default|GetSkeletalMesh) (CallFunction|RInterptoQuaternion (Transformation|GetWorldRotation (Variables|Default|GetSkeletalMesh)) (Math|Rotator|MakeRotator (.roll _returnvalue) (.pitch _returnvalue) (.yaw (Math|Rotator|FindLookatRotation _returnvalue_2 (Variables|Default|GetTargetPosition)))) (Utilities|Time|GetWorldDeltaSeconds) 4e+02) false false))

(fn SetOrderNumber
  (params (OrderNumber :type EnemyOrderEnum%20Enum :default "NewEnumerator0"))
  (bind _output_get (Variables|Default|SetOrderNumber OrderNumber))
  (Variables|Default|SetMoveStop false)
  (bind _output_get_2 (Variables|Default|SetCollisionType "NoCollision"))
  (Collision|SetCollisionEnabled (Variables|コンポーネント|GetBox) _output_get_2)
  (switch Utilities|FlowControl|Switch|SwitchonEnemyOrderEnum _output_get ; 命令対象が動かない物体ならターゲットポジションをセットする
    (:NewEnumerator1
      ;[1 1 1] 巣の周辺の位置をランダムで取得
      (bind _outactors (Actor|GetAllActorsOfClass "/Game/Main/Blueprints/Enemy/NestOyaclass.NestOyaclass_C"))
      (for _array_element _outactors
        (bind _targetpoint (Default|GetEnemyTargetPoint _array_element))
        (Variables|Default|SetTargetPosition _targetpoint)
        (Variables|Default|SetAttackMode false)))
    (:NewEnumerator2
      ;[1 1 1] 対象の位置を取得
      (bind _outactors_2 (Actor|GetAllActorsOfClass "/Game/Main/Blueprints/PlayerCastle.PlayerCastle_C"))
      (for _array_element_2 _outactors_2
        (bind _targetpoint_2 (Default|GetCastleTargetPoint _array_element_2))
        (Variables|Default|SetTargetPosition _targetpoint_2)
        (Variables|Default|SetAttackMode false)))
    (:NewEnumerator3
      ;[1 1 1] 対象の位置を取得
      (bind _outactors_3 (Actor|GetAllActorsOfClass "/Game/Main/Blueprints/Enemy/NestOyaclass.NestOyaclass_C"))
      (for _array_element_3 _outactors_3
        (Variables|Default|SetTargetPosition (Transformation|GetWorldLocation (Variables|/Game/Main/Blueprints/Enemy/NestOyaclass.NestOyaclass_C|GetStaticMesh _array_element_3)))
        (Variables|Default|SetAttackMode false)
        (Variables|Default|SetAttackMode false)))))

(fn RInterptoQuaternion
  (params (Current :type Rotator) (target :type Rotator) (DataTime :type Float%20%28single-precision%29) (InterpSpeed :type Float%20%28single-precision%29))
  (Utilities|FlowControl|Sequence
    (:then_0
      (LocalVariables|SetTargetRotator target)
      (LocalVariables|SetRotatorAngle (* DataTime InterpSpeed)) ; このフレームでの回転量
      (LocalVariables|SetCurrentXVec (Math|Rotator|GetRotationXVector Current))
      (LocalVariables|SetTargetXVec (Math|Rotator|GetRotationXVector target))
      (LocalVariables|SetAxis (Math|Vector|CrossProduct (LocalVariables|GetCurrentXVec) (LocalVariables|GetTargetXVec))) ; 回転軸
    )
    (:then_1
      ;[1 1 1] 回転量よりなす角が小さければ、Targetの回転を返す
      (if (<= (Class|KismetMathLibrary|DegAcos (Math|Vector|DotProduct (LocalVariables|GetCurrentXVec) (LocalVariables|GetTargetXVec))) (LocalVariables|GetRotatorAngle))
        (return (LocalVariables|GetTargetRotator))
        (else
          ;[1 1 1] クォータニオンによる回転
          (return (Math|Conversions|RotationFromXVector (Math|Vector|RotateVectorAroundAxis (LocalVariables|GetCurrentXVec) (LocalVariables|GetRotatorAngle) (LocalVariables|GetAxis)))))))))

(fn Rotate
  (params (TargetPosition :type Vector) (RotateSpeed :type Float%20%28single-precision%29))
  (bind _skeletalmesh (Variables|Default|GetSkeletalMesh))
  (bind _returnvalue (Transformation|GetWorldRotation _skeletalmesh))
  ;[1 1 1] 徐々にターゲットの方に回転させる
  (Transformation|SetWorldRotation (Variables|Default|GetSkeletalMesh) (CallFunction|RInterptoQuaternion (Transformation|GetWorldRotation (Variables|Default|GetSkeletalMesh)) (Math|Rotator|MakeRotator (.roll _returnvalue) (.pitch _returnvalue) (.yaw (Math|Rotator|FindLookatRotation (Transformation|GetWorldLocation (Variables|Default|GetSkeletalMesh)) TargetPosition))) (Utilities|Time|GetWorldDeltaSeconds) RotateSpeed) false false))

(fn SetCollision
  (params (CollisionON :type Boolean) (Collision :type Primitive%20Component%20Object%20Reference))
  (if CollisionON
    (Rendering|SetVisibility Collision true false)
    (Collision|SetCollisionEnabled Collision "QueryOnly")
    (else
      (Rendering|SetVisibility Collision false false)
      (Collision|SetCollisionEnabled Collision "NoCollision"))))

(fn GetYusyaPosition
  (LocalVariables|SetYusyaTargetPosition "0, 0, 0")
  (LocalVariables|SetYusyaTimeDistance 0.0)
  (LocalVariables|SetYusyaNearDistance 0.0)
  (bind _outactors (Actor|GetAllActorsOfClass "/Game/Main/Blueprints/Yusya/YusyaOyaclass.YusyaOyaclass_C"))
  ;[1 1 1] 一番近い勇者の場所を得る
  (for _array_element _outactors
    (LocalVariables|SetYusyaTimeDistance (Math|Vector|Distance(Vector) (Transformation|GetWorldLocation (Variables|/Game/Main/Blueprints/Yusya/YusyaOyaclass.YusyaOyaclass_C|GetSkeletalMesh _array_element)) (Transformation|GetWorldLocation (Variables|Default|GetSkeletalMesh))))
    (if (== (LocalVariables|GetYusyaNearDistance) 0.0)
      (LocalVariables|SetYusyaNearDistance (LocalVariables|GetYusyaTimeDistance) :!label _label)
      (LocalVariables|SetYusyaTargetPosition (Transformation|GetWorldLocation (Variables|/Game/Main/Blueprints/Yusya/YusyaOyaclass.YusyaOyaclass_C|GetSkeletalMesh _array_element)))
      (elif (> (LocalVariables|GetYusyaNearDistance) (LocalVariables|GetYusyaTimeDistance))
        (goto _label))))
  ;[1 1 1] 勇者がいないときは巣を守る
  (if (== (LocalVariables|GetYusyaNearDistance) 0.0)
    (return (Variables|Default|GetStartNestPosition))
    (else
      (return (LocalVariables|GetYusyaTargetPosition)))))

(fn TargetPointCheck
  (params (Length :type Float%20%28single-precision%29))
  ;[1 1 1] ターゲットの位置に着いているか判定
  (if (not (Variables|Default|GetAttackMode))
    (if (>= (+ (.x (Variables|Default|GetTargetPosition)) Length) (.x (Transformation|GetWorldLocation (Variables|Default|GetSkeletalMesh))))
      (if (<= (- (.x (Variables|Default|GetTargetPosition)) Length) (.x (Transformation|GetWorldLocation (Variables|Default|GetSkeletalMesh))))
        (if (>= (+ (.y (Variables|Default|GetTargetPosition)) Length) (.y (Transformation|GetWorldLocation (Variables|Default|GetSkeletalMesh))))
          (if (<= (- (.y (Variables|Default|GetTargetPosition)) Length) (.y (Transformation|GetWorldLocation (Variables|Default|GetSkeletalMesh))))
            (Transformation|SetWorldLocation (Variables|Default|GetSkeletalMesh) (Variables|Default|GetTargetPosition) false false)
            (Variables|Default|SetMoveStop true)
            (else
              (Variables|Default|SetMoveStop false)))
          (else
            (Variables|Default|SetMoveStop false)))
        (else
          (Variables|Default|SetMoveStop false)))
      (else
        (Variables|Default|SetMoveStop false)))))

(fn YusyaCastleRotate
  (params (self2 :type Scene%20Component%20Object%20Reference))
  (bind _skeletalmesh (Variables|Default|GetSkeletalMesh))
  (bind _returnvalue (Transformation|GetWorldRotation _skeletalmesh))
  (Transformation|SetWorldRotation (Variables|Default|GetSkeletalMesh) (CallFunction|RInterptoQuaternion (Transformation|GetWorldRotation (Variables|Default|GetSkeletalMesh)) (Math|Rotator|MakeRotator (.roll _returnvalue) (.pitch _returnvalue) (.yaw (Math|Rotator|FindLookatRotation (Transformation|GetWorldLocation self2) (Variables|Default|GetYusyaCastlePosition)))) (Utilities|Time|GetWorldDeltaSeconds) 1.2e+02) false false))