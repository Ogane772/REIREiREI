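; Function that steps a Current rotator toward Target at a constant angular speed of InterpSpeed degrees per unit of DataTime, as an RInterp-style helper.
; It rotates Current's forward vector about the cross product of both forward vectors, avoiding per-component Euler interpolation.
; It returns Target once the remaining angle fits within the step; otherwise it rebuilds the rotator from the X vector alone, so roll is not interpolated.
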(fn RInterptoQuaternionFunction
  (params (Current :type Rotator) (target :type Rotator) (DataTime :type Float%20%28single-precision%29) (InterpSpeed :type Float%20%28single-precision%29))
  (Utilities|FlowControl|Sequence
    (:then_0
      (LocalVariables|SetTargetRotator target)
      (LocalVariables|SetRotatorAngle (* DataTime InterpSpeed)) ; このフレームでの回転量
      (LocalVariables|SetCurrentXVec (Math|Rotator|GetRotationXVector Current))
      (LocalVariables|SetTargetXVec (Math|Rotator|GetRotationXVector target))
      (LocalVariables|SetAxis (Math|Vector|CrossProduct (LocalVariables|GetCurrentXVec) (LocalVariables|GetTargetXVec))) ; 回転軸
    )
    (:then_1
      ;[1 1 1] 回転量よりなす角が小さければ、Targetの回転を返す
      (if (<= (Class|KismetMathLibrary|DegAcos (Math|Vector|DotProduct (LocalVariables|GetCurrentXVec) (LocalVariables|GetTargetXVec))) (LocalVariables|GetRotatorAngle))
        (return (LocalVariables|GetTargetRotator))
        (else
          ;[1 1 1] クォータニオンによる回転
          (return (Math|Conversions|RotationFromXVector (Math|Vector|RotateVectorAroundAxis (LocalVariables|GetCurrentXVec) (LocalVariables|GetRotatorAngle) (LocalVariables|GetAxis)))))))))